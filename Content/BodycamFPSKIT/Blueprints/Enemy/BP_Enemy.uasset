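; Enemy character Blueprint that takes damage, reacts physically to hits and ragdolls on death.
; Any damage and radial damage reduce Health; lethal normal damage plays a death sound, while lethal radial damage ragdolls with an impulse.
; HitReaction briefly simulates physics below the struck bone, then a timeline blends it back out.
; Ragdoll scales the hit impulse differently for headshots and disables capsule collision.
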(event Custom|HitReaction
  (params (InBoneName :type Name :default "Pelvis") (Velocity :type Vector))
  (bind _mesh (Variables|Character|GetMesh))
  ;[0 0 0] PROCEDURAL HIT CALCULATION
  (if (== InBoneName "pelvis")
    (if (<= (Variables|Player|GetHealth) 0.0)
      (CallFunction|Ragdoll 5e+01 3.5))
    (else
      (Utilities|FlowControl|DoOnce false :!label _label
        (:Completed
          (Variables|HitCalculation|SetHitBoneName InBoneName)
          (Variables|HitCalculation|SetImpulseVel Velocity)
          (if (<= (Variables|Player|GetHealth) 0.0)
            (CallFunction|Ragdoll 5e+01 3.5)
            (else
              (Class|SkeletalMeshComponent|SetAllBodiesBelowSimulatePhysics _mesh (Variables|HitCalculation|GetHitBoneName) true true)
              (Class|SkeletalMeshComponent|SetAllBodiesBelowPhysicsBlendWeight _mesh (Variables|HitCalculation|GetHitBoneName) 1.0 true true)
              (Class|SkeletalMeshComponent|AddImpulsetoAllBodiesBelow (Variables|Character|GetMesh) (* (Variables|HitCalculation|GetImpulseVel) (Math|Float|SelectFloat 1.0 0.1 (== (Variables|HitCalculation|GetHitBoneName) "head"))) (Variables|HitCalculation|GetHitBoneName) true true)
              (bind _physics (Timeline|SimulateOff PlayFromStart)
                (:Update
                  (Class|SkeletalMeshComponent|SetAllBodiesBelowPhysicsBlendWeight (Variables|Character|GetMesh) (Variables|HitCalculation|GetHitBoneName) (Math|Float|Lerp 1.0 0.0 _physics) true true)
                  (if (Variables|Player|GetDead)
                    (Class|SkeletalMeshComponent|SetAllBodiesBelowSimulatePhysics (Variables|Character|GetMesh) (Variables|HitCalculation|GetHitBoneName) false true :!label _label_2)
                    (CallFunction|Ragdoll 0.15 0.15)))
                (:Finished
                  (Class|SkeletalMeshComponent|SetAllBodiesBelowSimulatePhysics (Variables|Character|GetMesh) (Variables|HitCalculation|GetHitBoneName) false true)
                  (if (Variables|Player|GetDead)
                    (goto _label_2)
                    (else
                      (goto _label Reset))))))))))))

(event Game|Damage|EventRadialDamage
  (params (DamageReceived :type Float%20%28single-precision%29) (DamageType :type Damage%20Type%20Object%20Reference) (Origin :type Vector :default "0, 0, 0") (HitInfo :type Hit%20Result%20Structure%20%28by%20ref%29) (InstigatedBy :type Controller%20Object%20Reference) (DamageCauser :type Actor%20Object%20Reference))
  (bind _mesh (Variables|Character|GetMesh))
  ;[0 0 0] DAMAGE
  (bind _output_get (Variables|Player|SetHealth (- (Variables|Player|GetHealth) DamageReceived)))
  (if (<= _output_get 0.0)
    (Variables|Player|SetDead true)
    (Physics|SetSimulatePhysics _mesh true)
    (Physics|AddImpulseatLocation (Variables|Character|GetMesh) "1000.000000,1000.000000,1000.000000" "0, 0, 0" "pelvis")
    (Collision|SetCollisionProfileName _mesh "Ragdoll" true :!class /Script/Engine.PrimitiveComponent)
    (Collision|SetCollisionEnabled (Variables|Collision|GetCapsuleComponent) "NoCollision")))

(event Game|Damage|EventAnyDamage
  (params (Damage :type Float%20%28single-precision%29) (DamageType :type Damage%20Type%20Object%20Reference) (InstigatedBy :type Controller%20Object%20Reference) (DamageCauser :type Actor%20Object%20Reference))
  ;[0 0 0] DAMAGE
  (bind _output_get (Variables|Player|SetHealth (- (Variables|Player|GetHealth) Damage)))
  (if (<= _output_get 0.0)
    (Variables|Player|SetDead true)
    (Audio|PlaySound2D "/Game/BodycamFPSKIT/Audio/Character/DeadEffect.DeadEffect" 1.0 1.0 0.1 0 0 false)
    (Audio|PlaySound2D "/Game/BodycamFPSKIT/Audio/Character/DeadEffect.DeadEffect" 1.0 1.0 0.25 0 0 false)
    (Audio|PlaySound2D "/Game/BodycamFPSKIT/Audio/Character/DeadEffect.DeadEffect" 1.0 1.0 0.3 0 0 false)))

(fn ConstructionScript)

(fn Ragdoll
  (params (ImpulseStrenghtHeadshot :type Float%20%28double-precision%29) (ImpulseStrenght :type Float%20%28double-precision%29))
  (bind _mesh (Variables|Character|GetMesh))
  (Physics|SetSimulatePhysics _mesh true)
  (Physics|AddImpulseatLocation (Variables|Character|GetMesh) (* (Variables|HitCalculation|GetImpulseVel) (* (Math|Float|SelectFloat ImpulseStrenghtHeadshot ImpulseStrenght (== (Variables|HitCalculation|GetHitBoneName) "head")) 0.05)) "0, 0, 0" (Variables|HitCalculation|GetHitBoneName))
  (Collision|SetCollisionProfileName _mesh "Ragdoll" true :!class /Script/Engine.PrimitiveComponent)
  (Collision|SetCollisionEnabled (Variables|Collision|GetCapsuleComponent) "NoCollision"))