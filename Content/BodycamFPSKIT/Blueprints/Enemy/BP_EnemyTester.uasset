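; BP_EnemyTester is a test actor that spawns and respawns BP_Enemy instances in the Bodycam FPS kit.
; On BeginPlay it spawns one enemy at each of its four Scene component transforms and stores them in EnemiesSpawned.
; RespawnEnemies, guarded by a DoOnce that resets afterwards, destroys the valid stored enemies and spawns a new set.
; The array is appended to on each spawn and never cleared.
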(event Custom|EnemySpawn
  (for _array_element (Utilities|Array|MakeArray (Variables|Default|GetScene) (Variables|Default|GetScene1) (Variables|Default|GetScene2) (Variables|Default|GetScene3))
    (bind _returnvalue (Game|SpawnActorfromClass "/Game/BodycamFPSKIT/Blueprints/Enemy/BP_Enemy.BP_Enemy_C" (Transformation|GetWorldTransform _array_element) "Undefined" "MultiplyWithRoot" 0 0))
    (Utilities|Array|Add (Variables|Default|GetEnemiesSpawned) _returnvalue)))

(event Custom|RespawnEnemies
  (Utilities|FlowControl|DoOnce false :!label _label
    (:Completed
      (for _array_element (Variables|Default|GetEnemiesSpawned)
        (Utilities|IsValid _array_element
          (:Is%20Valid
            (Actor|DestroyActor _array_element))))
      (CallFunction|EnemySpawn)
      (goto _label Reset))))

(event EventBeginPlay
  (CallFunction|EnemySpawn))

(fn ConstructionScript)