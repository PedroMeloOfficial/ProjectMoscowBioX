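; Actor component that lets its owning character climb BP_Ladder actors in the Bodycam FPS kit.
; Overlapping a ladder switches movement to Flying, with fly speed and braking set at BeginPlay, and leaving it restores Walking.
; ClimbMovement turns an input value into motion along the actor's up axis, choosing up or down from camera pitch against LookUpAngle.
; ReleaseLadder exits climbing early and applies a forward impulse.
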(event Custom|ClimbMovement
  (params (PitchValue :type Float%20%28double-precision%29))
  ;[1 0 0.8775] Climbing Movement
  (Variables|Default|SetlookingUp? (>= (.Pitch (Math|Vector|GetYawPitchfromVector (Math|Vector|GetForwardVector (Variables|Default|GetGame%20View%20Camera)))) (Variables|LadderSettings|GetLookUpAngle)))
  (Pawn|Input|AddMovementInput (Variables|/Script/Engine.Actor|GetInstigator (Variables|Default|GetOwner)) (Math|Vector|SelectVector (Transformation|GetActorUpVector (Variables|Default|GetOwner)) (* (Transformation|GetActorUpVector (Variables|Default|GetOwner)) -1) (Variables|Default|GetlookingUp?)) PitchValue false))

(event Custom|OnOwnerBeginOverlapped
  (params (Overlapped%20Actor :type Actor%20Object%20Reference) (Other%20Actor :type Actor%20Object%20Reference))
  ;[1 0 0.8775] Overlaps
  (if (== (Utilities|GetClass Other%20Actor) "/Game/BodycamFPSKIT/Blueprints/Interactables/Misc/BP_Ladder.BP_Ladder_C")
    (Pawn|Components|CharacterMovement|SetMovementMode (Variables|Default|GetOwnerMovementComponent) "MOVE_Flying" 0)
    (Variables|Default|SetisClimbing? true)))

(event Custom|OwnerEndOverlapped
  (params (OverlappedActor :type Actor%20Object%20Reference) (OtherActor :type Actor%20Object%20Reference))
  ;[1 0 0.8775] Initialize
  (CallFunction|OnOwnerEndOverlapped OverlappedActor OtherActor))

(event Custom|OnOwnerEndOverlapped
  (params (OverlappedActor :type Actor%20Object%20Reference) (OtherActor :type Actor%20Object%20Reference))
  ;[1 0 0.8775] Overlaps
  (if (== (Utilities|GetClass OtherActor) "/Game/BodycamFPSKIT/Blueprints/Interactables/Misc/BP_Ladder.BP_Ladder_C")
    (Pawn|Components|CharacterMovement|SetMovementMode (Variables|Default|GetOwnerMovementComponent) "MOVE_Walking" 0)
    (Variables|Default|SetisClimbing? false)))

(event Custom|ReleaseLadder
  ;[1 0 0.8775] Release Ladder
  (if (Variables|Default|GetisClimbing?)
    (Pawn|Components|CharacterMovement|SetMovementMode (Variables|Default|GetOwnerMovementComponent) "MOVE_Walking" 0)
    (Variables|Default|SetisClimbing? false)
    (Physics|AddImpulse (Variables|Default|GetOwnerMovementComponent) (* (Transformation|GetActorForwardVector (Variables|Default|GetOwner)) (Variables|LadderSettings|GetReleaseImpulseStrength)) false)))

(event Custom|OwnerBeginOverlapped
  (params (OverlappedActor :type Actor%20Object%20Reference) (OtherActor :type Actor%20Object%20Reference))
  ;[1 0 0.8775] Initialize
  (CallFunction|OnOwnerBeginOverlapped OverlappedActor OtherActor))

(event EventBeginPlay
  ;[1 0 0.8775] Initialize
  (Variables|Default|SetOwner (Components|GetOwner))
  (Collision|BindEventtoOnActorBeginOverlap (Variables|Default|GetOwner) (delegate Custom|OwnerBeginOverlapped))
  (Collision|BindEventtoOnActorEndOverlap (Variables|Default|GetOwner) (delegate Custom|OwnerEndOverlapped))
  (Variables|Default|SetOwnerMovementComponent (Actor|GetComponentbyClass (Variables|Default|GetOwner) "/Script/Engine.CharacterMovementComponent"))
  (Variables|/Script/Engine.CharacterMovementComponent|SetMaxFlySpeed (Variables|Default|GetOwnerMovementComponent) 2e+02)
  (Variables|/Script/Engine.CharacterMovementComponent|SetBrakingDecelerationFlying (Variables|Default|GetOwnerMovementComponent) 2e+03)
  (Variables|Default|SetGame%20View%20Camera (Actor|GetComponentbyClass (Variables|Default|GetOwner) "/Script/Engine.CameraComponent")))