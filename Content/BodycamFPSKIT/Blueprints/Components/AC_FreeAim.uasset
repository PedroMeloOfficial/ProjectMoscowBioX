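; Actor component that adds bodycam-style free aim, letting mouse input drift within a rotational deadzone.
; FreeAimComponent scales mouse input, accumulates it into per-axis rotations clamped to hip or aim limits, and optionally adds tilt.
; It smoothly lerps the passed effector component's relative rotation and returns an axis-remapped FreeAim transform.
; Tick is empty, and the EventGraph's delayed aim-limit reset is unconnected.
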(event EventTick
  (params (DeltaSeconds :type Float%20%28single-precision%29)))

(fn FreeAimComponent
  (params (EffectorComponent :type Scene%20Component%20Object%20Reference) (HorizontalMouse :type Float%20%28double-precision%29) (VerticalMouse :type Float%20%28double-precision%29) (Speed :type Float%20%28double-precision%29) (Aim :type Boolean) (IsActive :type Boolean))
  (if IsActive
    (Variables|InputValues|SetEffector%20Component EffectorComponent)
    (Variables|FreeAim|SetAim Aim)
    (Variables|InputValues|SetHorizontal%20Mouse (* HorizontalMouse Speed))
    (Variables|InputValues|SetVertical%20Mouse (* VerticalMouse Speed))
    (Variables|InputValues|SetDelta%20Time (Utilities|Time|GetWorldDeltaSeconds))
    (Utilities|FlowControl|Sequence
      (:then_0
        (Utilities|FlowControl|Sequence
          (:then_0
            (if (> (Variables|InputValues|GetHorizontal%20Mouse) 1.0)
              (Variables|InputValues|SetHorizontal%20Mouse 1.0)))
          (:then_1
            (if (< (Variables|InputValues|GetHorizontal%20Mouse) -1.0)
              (Variables|InputValues|SetHorizontal%20Mouse -1.0)))))
      (:then_1
        (if (Variables|FreeAim|GetEnableDeadzoneX)
          (Variables|FreeAim|SetRotX (Math|Rotator|MakeRotator (+ (* (Variables|InputValues|GetHorizontal%20Mouse) (Variables|FreeAim|GetStartSensitivity)) (.Roll (Math|Rotator|BreakRotator (Variables|FreeAim|GetRotX)))) (+ (* (Variables|InputValues|GetHorizontal%20Mouse) (Variables|FreeAim|GetStartSensitivity)) (.Pitch (Math|Rotator|BreakRotator (Variables|FreeAim|GetRotX)))) (+ (* (Variables|InputValues|GetHorizontal%20Mouse) (Variables|FreeAim|GetStartSensitivity)) (.Yaw (Math|Rotator|BreakRotator (Variables|FreeAim|GetRotX))))))
          (Variables|FreeAim|SetRotX (Math|Rotator|MakeRotator (Math|Float|ClampAngle (.Roll (Math|Rotator|BreakRotator (Variables|FreeAim|GetRotX))) (Math|Float|SelectFloat (Variables|FreeAim|GetMinRotX_Aim) (Variables|FreeAim|GetMinRotX) (Variables|FreeAim|GetAim)) (Math|Float|SelectFloat (Variables|FreeAim|GetMaxRotX_Aim) (Variables|FreeAim|GetMaxRotX) (Variables|FreeAim|GetAim))) (.Pitch (Math|Rotator|BreakRotator (Variables|FreeAim|GetRotX))) (.Yaw (Math|Rotator|BreakRotator (Variables|FreeAim|GetRotX)))))))
      (:then_2
        (if (Variables|FreeAim|GetEnableDeadzoneY)
          (Variables|FreeAim|SetRotY (Math|Rotator|MakeRotator (+ (* (Variables|InputValues|GetVertical%20Mouse) (Variables|FreeAim|GetStartSensitivity)) (.Roll (Math|Rotator|BreakRotator (Variables|FreeAim|GetRotY)))) (+ (* (Variables|InputValues|GetVertical%20Mouse) (Variables|FreeAim|GetStartSensitivity)) (.Pitch (Math|Rotator|BreakRotator (Variables|FreeAim|GetRotY)))) (+ (* (Variables|InputValues|GetVertical%20Mouse) (Variables|FreeAim|GetStartSensitivity)) (.Yaw (Math|Rotator|BreakRotator (Variables|FreeAim|GetRotY))))))
          (Variables|FreeAim|SetRotY (Math|Rotator|MakeRotator (.Roll (Math|Rotator|BreakRotator (Variables|FreeAim|GetRotY))) (.Pitch (Math|Rotator|BreakRotator (Variables|FreeAim|GetRotY))) (Math|Float|ClampAngle (.Yaw (Math|Rotator|BreakRotator (Variables|FreeAim|GetRotY))) (Math|Float|SelectFloat (Variables|FreeAim|GetMinRotY_Aim) (Variables|FreeAim|GetMinRotY) (Variables|FreeAim|GetAim)) (Math|Float|SelectFloat (Variables|FreeAim|GetMaxRotY_Aim) (Variables|FreeAim|GetMaxRotY) (Variables|FreeAim|GetAim)))))))
      (:then_3
        (if (Variables|FreeAim|GetEnableTilt)
          (Variables|FreeAim|SetTiltAroundZ (Math|Rotator|MakeRotator 0.0 0.0 (* (Variables|InputValues|GetVertical%20Mouse) (Variables|FreeAim|GetTiltingAngle))))
          (Variables|FreeAim|SetTiltAroundX (Math|Rotator|MakeRotator 0.0 (* (Variables|InputValues|GetHorizontal%20Mouse) (Variables|FreeAim|GetTiltingAngle)) 0.0))
          (Variables|FreeAim|SetTiltTargetRot (Math|Rotator|MakeRotator (.pitch (Variables|FreeAim|GetTiltAroundX)) 0.0 (.yaw (Variables|FreeAim|GetTiltAroundX))))
          (Transformation|SetRelativeRotation (Variables|InputValues|GetEffector%20Component) (Math|Rotator|Lerp(Rotator) (Variables|/Script/Engine.SceneComponent|GetRelativeRotation (Variables|InputValues|GetEffector%20Component)) (Variables|FreeAim|GetTiltTargetRot) (* (Variables|InputValues|GetDelta%20Time) (Variables|FreeAim|GetSmoothRotation))) false false)))
      (:then_4
        (Variables|FreeAim|SetDeadZoneTargetRot (Math|Rotator|MakeRotator (.roll (Variables|FreeAim|GetRotX)) 0.0 (.yaw (Variables|FreeAim|GetRotY))))
        (Transformation|SetRelativeRotation (Variables|InputValues|GetEffector%20Component) (Math|Rotator|Lerp(Rotator) (Variables|/Script/Engine.SceneComponent|GetRelativeRotation (Variables|InputValues|GetEffector%20Component)) (Variables|FreeAim|GetDeadZoneTargetRot) (* (Variables|InputValues|GetDelta%20Time) (Variables|FreeAim|GetSmoothRotation))) false false)
        (bind _output_get (Variables|FreeAim|SetFinalDeadzoneAimRotation (Variables|/Script/Engine.SceneComponent|GetRelativeRotation (Variables|InputValues|GetEffector%20Component))))
        (bind _output_get_2 (Variables|FreeAim|SetFreeAim (Math|Transform|MakeTransform (Math|Vector|MakeVector 0.0 0.0 0.0) (Math|Rotator|MakeRotator (* (.Yaw (Math|Rotator|BreakRotator _output_get)) -1.0) 0.0 (.Roll (Math|Rotator|BreakRotator _output_get))))))
        (return _output_get_2)))))