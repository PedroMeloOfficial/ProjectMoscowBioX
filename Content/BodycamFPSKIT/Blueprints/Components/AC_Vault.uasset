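; Character component for the bodycam FPS kit that handles mantling onto and vaulting over obstacles.
; While idle, Tick runs two downward capsule traces ahead, checking height, walkable slope and capsule clearance to pick a landing and mantle or vault-over.
; The Vault event starts the move and optionally triggers the ABP_Manny animation.
; Tick then moves the actor without sweep along a cubic Bezier built from nested lerps, shaped by vault type.
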(event Custom|Vault
  (params (PlayAnim :type Boolean))
  (bind _as_character (Variables|Default|GetAs%20Character))
  (Variables|Default|SetProgress 0.0)
  (Variables|Default|SetStartingLocation (Transformation|GetActorLocation _as_character))
  (Variables|Default|SetVaultState "NewEnumerator2")
  (if PlayAnim
    (bind _asabp_manny (Utilities|Casting|CastToABP_Manny (Components|SkeletalMesh|GetAnimInstance (Variables|/Script/Engine.Character|GetMesh _as_character))))
    (Default|VaultAnim _asabp_manny)))

(event EventBeginPlay
  (bind _ascharacter (Utilities|Casting|CastToCharacter (Components|GetOwner)))
  (bind _output_get (Variables|Default|SetAs%20Character _ascharacter))
  (Variables|Default|SetMesh (Variables|/Script/Engine.Character|GetMesh _output_get))
  (Variables|Default|SetCharacter%20Movement (Variables|/Script/Engine.Character|GetCharacterMovement _output_get)))

(event EventTick
  (params (DeltaSeconds :type Float%20%28single-precision%29))
  (Utilities|SwitchVaultState
    (:NotVault
      (bind (_result _endinglocation _isvaultover) (CallFunction|CanVault))
      (if _result
        (Variables|Default|SetEndingLocation _endinglocation)
        (bind _output_get (Variables|Default|SetIs%20Vault%20Over _isvaultover))
        (if _output_get
          (Variables|Default|SetVaultSpeed 0.45)
          (else
            (Variables|Default|SetVaultSpeed 0.45)))))
    (:Vaulting
      (CallFunction|TickVault DeltaSeconds))))

(fn CanVault
  (bind _as_character (Variables|Default|GetAs%20Character))
  (bind _as_character_2 (Variables|Default|GetAs%20Character))
  (bind _returnvalue (Transformation|GetActorLocation _as_character))
  (bind _returnvalue_2 (Transformation|GetActorLocation _as_character_2))
  (bind _returnvalue_3 (Transformation|GetActorForwardVector _as_character))
  (bind _returnvalue_4 (Transformation|GetActorForwardVector _as_character_2))
  (bind _returnvalue_5 (* _returnvalue_3 1.4e+02))
  (bind _returnvalue_6 (* _returnvalue_4 7e+01))
  (bind _returnvalue_7 (+ _returnvalue _returnvalue_5))
  (bind _returnvalue_8 (+ _returnvalue_2 _returnvalue_6))
  (if (Utilities|Enum|Equal(Enum) (Variables|Default|GetVaultState) "NewEnumerator0")
    (LocalVariables|SetCapsule%28local%29 (Variables|/Script/Engine.Character|GetCapsuleComponent (Variables|Default|GetAs%20Character)))
    (bind (_outhit _returnvalue_9) (Collision|CapsuleTraceByChannel (+ _returnvalue_8 (Math|Vector|MakeVector 0.0 0.0 (Components|Capsule|GetScaledCapsuleHalfHeight (LocalVariables|GetCapsule%28local%29)))) (- _returnvalue_8 (Math|Vector|MakeVector 0.0 0.0 (Components|Capsule|GetScaledCapsuleHalfHeight (LocalVariables|GetCapsule%28local%29)))) 1e+01 1e+01 "TraceTypeQuery1" false (Utilities|Array|MakeArray (Variables|Default|GetAs%20Character)) "None"))
    (if _returnvalue_9
      (bind (_result _endinglocation) (CallFunction|CanVaulttoHit (LocalVariables|GetCapsule%28local%29) _outhit))
      (if _result
        (LocalVariables|SetVaultLoc%28local%29 _endinglocation)
        (bind (_outhit_2 _returnvalue_10) (Collision|CapsuleTraceByChannel (+ _returnvalue_7 (Math|Vector|MakeVector 0.0 0.0 (Components|Capsule|GetScaledCapsuleHalfHeight (LocalVariables|GetCapsule%28local%29)))) (- _returnvalue_7 (Math|Vector|MakeVector 0.0 0.0 (Components|Capsule|GetScaledCapsuleHalfHeight (LocalVariables|GetCapsule%28local%29)))) 1e+01 1e+01 "TraceTypeQuery1" false (Utilities|Array|MakeArray (Variables|Default|GetAs%20Character)) "None"))
        (if _returnvalue_10
          (bind (_result_2 _endinglocation_2) (CallFunction|CanVaultOvertoHit (LocalVariables|GetCapsule%28local%29) _outhit_2))
          (if _result_2
            (return true _endinglocation_2 true)
            (else
              _)))
        (return true (LocalVariables|GetVaultLoc%28local%29) false)
        (else
          _)))
    (return false "0, 0, 0" false)
    (else
      (return false "0, 0, 0" false))))

(fn CanVaulttoHit
  (params (Capsule :type Capsule%20Component%20Object%20Reference) (Hit :type Hit%20Result%20Structure))
  (bind _as_character (Variables|Default|GetAs%20Character))
  (bind _capsulecomponent (Variables|/Script/Engine.Character|GetCapsuleComponent _as_character))
  (bind _returnvalue (Components|Capsule|GetScaledCapsuleHalfHeight _capsulecomponent))
  (bind _returnvalue_2 (Components|Capsule|GetScaledCapsuleRadius _capsulecomponent))
  (Utilities|FlowControl|Sequence
    (:then_0
      ;[1 1 1] Check the ledge height
      (if (not (Math|Float|InRange(Float) (- (.Z (Math|Vector|BreakVector (.location Hit))) (.Z (Math|Vector|BreakVector (.traceend Hit)))) (Variables|Default|GetMinVaultingHeight) (Variables|Default|GetMaxVaultingHeight)))
        (return false "0, 0, 0")))
    (:then_1
      ;[1 1 1] Check the surface is walkable
      (if (< (.Z (Math|Vector|BreakVector (.normal Hit))) (Class|CharacterMovementComponent|GetWalkableFloorZ (Variables|Default|GetCharacter%20Movement)))
        (return false "0, 0, 0")))
    (:then_2
      ;[1 1 1] Check the space for the character on top
      (bind _output_get (LocalVariables|SetEndingLocation%28local%29 (+ (.location Hit) (Math|Vector|MakeVector 0.0 0.0 _returnvalue))))
      (bind _result (CallFunction|CheckCapsuleCollision (+ _output_get (Math|Vector|MakeVector 0.0 0.0 _returnvalue_2)) _returnvalue _returnvalue_2 false))
      (if _result
        (return false "0, 0, 0")))
    (:then_3
      (return true (LocalVariables|GetEndingLocation%28local%29)))))

(fn CanVaultOvertoHit
  (params (Capsule :type Capsule%20Component%20Object%20Reference) (Hit :type Hit%20Result%20Structure))
  (bind _as_character (Variables|Default|GetAs%20Character))
  (bind _capsulecomponent (Variables|/Script/Engine.Character|GetCapsuleComponent _as_character))
  (bind _returnvalue (Components|Capsule|GetScaledCapsuleHalfHeight _capsulecomponent))
  (Utilities|FlowControl|Sequence
    (:then_0
      ;[1 1 1] Check the ledge height
      (if (not (Math|Float|InRange(Float) (- (.Z (Math|Vector|BreakVector (.location Hit))) (.Z (Math|Vector|BreakVector (.traceend Hit)))) 0.0 5e+01))
        (return false "0, 0, 0")))
    (:then_1
      ;[1 1 1] Check the surface is walkable
      (if (< (.Z (Math|Vector|BreakVector (.normal Hit))) (Class|CharacterMovementComponent|GetWalkableFloorZ (Variables|Default|GetCharacter%20Movement)))
        (return false "0, 0, 0")))
    (:then_2
      ;[1 1 1] Check the space for the character on top
      (bind _output_get (LocalVariables|SetEndingLocation%28local%29 (+ (.location Hit) (Math|Vector|MakeVector 0.0 0.0 _returnvalue))))
      (bind _result (CallFunction|CheckCapsuleCollision (+ _output_get (Math|Vector|MakeVector 0.0 0.0 0.0)) _returnvalue (Components|Capsule|GetScaledCapsuleRadius _capsulecomponent) false))
      (if _result
        (return false "0, 0, 0")))
    (:then_3
      (return true (LocalVariables|GetEndingLocation%28local%29)))))

(fn CheckCapsuleCollision
  (params (Center :type Vector) (HalfHeight :type Float%20%28double-precision%29) (Radius :type Float%20%28double-precision%29) (DrawDebug :type Boolean))
  (Utilities|FlowControl|Sequence
    (:then_0
      (if DrawDebug
        (Rendering|Debug|DrawDebugCapsule Center HalfHeight Radius "0, 0, 0" "(R=1.000000,G=1.000000,B=1.000000,A=1.000000)" 0.0 3.0)))
    (:then_1
      (bind _returnvalue (Collision|CapsuleOverlapActors Center Radius HalfHeight (Utilities|Array|MakeArray "ObjectTypeQuery1" "ObjectTypeQuery2" "ObjectTypeQuery4" "ObjectTypeQuery5" "ObjectTypeQuery6") "/Script/Engine.Actor" (Utilities|Array|MakeArray (Variables|Default|GetAs%20Character))))
      (return _returnvalue))))

(fn TickVault
  (params (DeltaSeconds :type Float%20%28double-precision%29))
  (bind _startinglocation (Variables|Default|GetStartingLocation))
  (bind _endinglocation (Variables|Default|GetEndingLocation))
  (Utilities|FlowControl|Sequence
    (:then_0
      (Variables|Default|SetProgress (Math|Float|Clamp(Float) (+ (Variables|Default|GetProgress) (/ DeltaSeconds (Variables|Default|GetVaultSpeed)))))
      (Transformation|SetActorLocation (Variables|Default|GetAs%20Character) (CallFunction|BezierLerp4Point _startinglocation (+ _startinglocation (Math|Vector|RotateVector (Math|Vector|SelectVector (Math|Vector|MakeVector 0.0 45.0 8e+01) (Math|Vector|MakeVector 25.0 0.0 1e+02) (Variables|Default|GetIs%20Vault%20Over)) (Transformation|GetActorRotation (Variables|Default|GetAs%20Character)))) (+ _endinglocation (Math|Vector|RotateVector (Math|Vector|SelectVector (Math|Vector|MakeVector 0.0 65.0 7e+01) (Math|Vector|MakeVector 0.0 0.0 0.0) (Variables|Default|GetIs%20Vault%20Over)) (Transformation|GetActorRotation (Variables|Default|GetAs%20Character)))) _endinglocation (Math|Float|Clamp(Float) (Variables|Default|GetProgress))) false false))
    (:then_1
      (if (>= (Variables|Default|GetProgress) 1.0)
        (Variables|Default|SetVaultState "NewEnumerator0")))))

(fn BezierLerp4Point
  (params (PStart :type Vector) (Offset_1 :type Vector :default "-1.500000,-2.000000,1.000000") (Offset_2 :type Vector) (PEnd :type Vector) (Alpha :type Float%20%28double-precision%29))
  (Utilities|FlowControl|Sequence
    (:then_0
      (LocalVariables|SetLerp_1 (Math|Vector|Lerp(Vector) PStart Offset_1 Alpha))
      (LocalVariables|SetLerp_2 (Math|Vector|Lerp(Vector) Offset_1 Offset_2 Alpha))
      (LocalVariables|SetLerp_3 (Math|Vector|Lerp(Vector) Offset_2 PEnd Alpha)))
    (:then_1
      (LocalVariables|SetLerp_4 (Math|Vector|Lerp(Vector) (LocalVariables|GetLerp_1) (LocalVariables|GetLerp_2) Alpha))
      (LocalVariables|SetLerp_5 (Math|Vector|Lerp(Vector) (LocalVariables|GetLerp_2) (LocalVariables|GetLerp_3) Alpha)))
    (:then_2
      (return (Math|Vector|Lerp(Vector) (LocalVariables|GetLerp_4) (LocalVariables|GetLerp_5) Alpha)))))