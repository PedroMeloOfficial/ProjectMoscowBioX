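; Base weapon Blueprint for throwable grenades held by the player, with one grenade moved from the MaxAmmo reserve into the hand.
; Firing stops running, then chains pin pull, throw and reload through delays, several timed from animation lengths.
; The throw spawns BP_GranadeProjectile near the right-hand socket and applies camera-forward, upward and angular impulses.
; Reload restores and refills the held mesh, clearing it when no grenades remain.
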(event Custom|ThrowGranade
  (bind _playerref (Variables|Default|GetPlayerRef))
  (bind _playerref_2 (Variables|Default|GetPlayerRef))
  (bind _returnvalue (Transformation|GetActorUpVector _playerref))
  (bind _firstpersoncamera (Variables|/Game/BodycamFPSKIT/Blueprints/BP_FPCharacter.BP_FPCharacter_C|GetFirstPersonCamera _playerref))
  (bind _mesh (Variables|/Script/Engine.Character|GetMesh _playerref))
  (bind _returnvalue_2 (* _returnvalue 5.5e+02))
  (bind _returnvalue_3 (Transformation|GetSocketTransform _mesh "hand_r" "RTS_World"))
  (bind _returnvalue_4 (Transformation|GetWorldRotation _firstpersoncamera))
  (bind _returnvalue_5 (Math|Vector|GetForwardVector _returnvalue_4))
  (bind _returnvalue_6 (* _returnvalue_5 1.35e+03))
  (bind _returnvalue_7 (+ _returnvalue_6 _returnvalue_2))
  ;[0 0 0] THROW GRANADE
  (bind _playlength (Default|PlayAnimation (Variables|/Game/BodycamFPSKIT/Blueprints/BP_FPCharacter.BP_FPCharacter_C|GetAC_ProceduralAnimation _playerref_2) (Variables|/Script/Engine.Character|GetMesh _playerref_2) "/Game/BodycamFPSKIT/Character/Animations/WeaponAnims/Granade/Anim_Arms_Granade_Throw.Anim_Arms_Granade_Throw" 1 1.0 0.0 1.0 "arms"))
  (Utilities|FlowControl|Sequence
    (:then_0
      (Utilities|FlowControl|Delay 0.7)
      (bind _returnvalue_8 (Game|SpawnActorfromClass "/Game/BodycamFPSKIT/Blueprints/Interactables/Granade/BP_GranadeProjectile.BP_GranadeProjectile_C" (Math|Transform|MakeTransform (+ (.location _returnvalue_3) (* (Math|Vector|GetForwardVector (.rotation _returnvalue_3)) 5e+01)) (Pawn|GetControlRotation _playerref :!class /Script/Engine.Pawn) "1.000000,1.000000,1.000000") "Undefined" "OverrideRootScale" 0 0))
      (Physics|AddImpulse (Variables|/Game/BodycamFPSKIT/Blueprints/Interactables/Granade/BP_GranadeProjectile.BP_GranadeProjectile_C|GetCollisionComponent _returnvalue_8) _returnvalue_7 "None" false)
      (Class|PrimitiveComponent|AddAngularImpulseinDegrees (Variables|/Game/BodycamFPSKIT/Blueprints/Interactables/Granade/BP_GranadeProjectile.BP_GranadeProjectile_C|GetCollisionComponent _returnvalue_8) (* _returnvalue_7 5e+01) "None" false))
    (:then_1
      (Utilities|FlowControl|Delay (- _playlength 1.0))
      (CallFunction|Reload))))

(event Custom|PinPullGranade
  (bind _pinpullanim (Variables|Animations|GetPinpullAnim))
  (bind _playerref (Variables|Default|GetPlayerRef))
  ;[0 0 0] PIN PULL GRANADE
  (bind _playlength (Default|PlayAnimation (Variables|/Game/BodycamFPSKIT/Blueprints/BP_FPCharacter.BP_FPCharacter_C|GetAC_ProceduralAnimation _playerref) (Variables|/Script/Engine.Character|GetMesh _playerref) "/Game/BodycamFPSKIT/Character/Animations/WeaponAnims/Granade/Anim_Arms_Granade_Pinpull.Anim_Arms_Granade_Pinpull" 1 1.0 0.05 0.05 "arms"))
  (Utilities|FlowControl|Sequence
    (:then_0
      (Audio|PlaySoundatLocation "/Game/BodycamFPSKIT/Audio/Character/Grenade_PinPull_2_Cue.Grenade_PinPull_2_Cue" (Transformation|GetActorLocation (Variables|Default|GetPlayerRef)) "0, 0, 0" 1.0 1.0 0.0 0 0 0 0)
      (Components|Animation|PlayAnimation (Variables|Default|GetItem_Mesh) _pinpullanim false)
      (Utilities|FlowControl|Delay (- (Variables|/Script/Engine.AnimSequenceBase|GetSequenceLength _pinpullanim) 0.1))
      (Components|SkinnedMesh|SetSkinnedAssetandUpdate (Variables|Default|GetItem_Mesh) (Variables|Default|GetMesh) false)
      (Utilities|FlowControl|Delay 0.7)
      (Rendering|SetVisibility (Variables|Default|GetItem_Mesh) false false)
      (CallFunction|SetAmmo (Math|Integer|Clamp(Integer) (- (Variables|Default|GetAmmoCount) 1) 0 99) (Variables|Default|GetMaxAmmo))
      (CallFunction|SetWeaponAmmoData false))
    (:then_1
      (Utilities|FlowControl|Delay (- _playlength 0.2))
      (CallFunction|ThrowGranade))))

(event Custom|AddGranade
  (bind _maxammo (Variables|Default|GetMaxAmmo))
  ;[0 0 0] ADD GRANADE TO HAND AND REMOVE ONE FROM MAX AMMO
  (CallFunction|SetAmmo (Math|Integer|SelectInt 0 (+ (Variables|Default|GetAmmoCount) 1) (== _maxammo 0)) (Math|Integer|Clamp(Integer) (- _maxammo 1) 0 99))
  (CallFunction|SetWeaponAmmoData false))

(event EventReload
  (bind _playerref (Variables|Default|GetPlayerRef))
  ;[0 0 0] RELOAD GRANADE
  (if (== (Variables|Default|GetAmmoCount) 0)
    (Default|PlayAnimation (Variables|/Game/BodycamFPSKIT/Blueprints/BP_FPCharacter.BP_FPCharacter_C|GetAC_ProceduralAnimation _playerref) (Variables|/Script/Engine.Character|GetMesh _playerref) "/Game/BodycamFPSKIT/Character/Animations/WeaponAnims/Granade/Anim_Arms_Granade_Recovery.Anim_Arms_Granade_Recovery" 1 1.0 0.1 0.1 "arms")
    (Utilities|FlowControl|Delay 0.1)
    (Rendering|SetVisibility (Variables|Default|GetItem_Mesh) true false)
    (Components|SkinnedMesh|SetSkinnedAssetandUpdate (Variables|Default|GetItem_Mesh) (Variables|Default|GetMesh) true)
    (Components|Animation|PlayAnimation (Variables|Default|GetItem_Mesh) (Variables|Default|GetEmptyWeaponAnim) false)
    (CallFunction|AddGranade)
    (Variables|Default|SetIsFire false)
    (if (== (Variables|Default|GetAmmoCount) 0)
      (Components|SkinnedMesh|SetSkinnedAssetandUpdate (Variables|Default|GetItem_Mesh) 0 false))))

(event EventBeginFire
  (bind _playerref (Variables|Default|GetPlayerRef))
  (bind _playerref_2 (Variables|Default|GetPlayerRef))
  ;[0 0 0] FIRE LOGIC
  (if (== (Variables|Default|GetAmmoCount) 0)
    (if (== (Variables|Default|GetMaxAmmo) 0)
      (Variables|/Game/BodycamFPSKIT/Blueprints/BP_FPCharacter.BP_FPCharacter_C|SetWeaponChangeHint _playerref "NO GRANADE")
      (Utilities|FlowControl|Delay 1.0)
      (Variables|/Game/BodycamFPSKIT/Blueprints/BP_FPCharacter.BP_FPCharacter_C|SetWeaponChangeHint _playerref ""))
    (else
      (if (Variables|/Game/BodycamFPSKIT/Blueprints/BP_FPCharacter.BP_FPCharacter_C|GetIsRun _playerref_2)
        (Default|ChangeMoveState _playerref_2 "NewEnumerator0"))
      (if (not (Variables|Default|GetIsFire))
        (Variables|Default|SetIsFire true)
        (CallFunction|PinPullGranade)))))

(event EventParentBeginPlay
  ;[0 0 0] BEGINPLAY
  (Utilities|FlowControl|DelayUntilNextTick)
  (if (== (Variables|Default|GetAmmoCount) 0)
    (if (> (Variables|Default|GetMaxAmmo) 0)
      (CallFunction|AddGranade)
      (else
        (Components|SkinnedMesh|SetSkinnedAssetandUpdate (Variables|Default|GetItem_Mesh) 0 false))))
  (Components|Animation|PlayAnimation (Variables|Default|GetItem_Mesh) (Variables|Default|GetEmptyWeaponAnim) false))

(fn ConstructionScript
  (|CallParentFunction))