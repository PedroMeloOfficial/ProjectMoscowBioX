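; BP_Weapon_EmptyHands is the unarmed weapon, giving the player a melee attack with bare hands.
; BeginFire plays a sound and one of two alternating arm animations through the player's procedural animation component, then runs a melee hit-scan trace.
; It sets LeftHandAlpha to full during the strike, then resets it after a short delay, which also releases the IsFire lock against overlapping attacks.
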(event EventBeginFire
  (bind _playerref (Variables|Default|GetPlayerRef))
  ;[0 0 0] FIRE LOGIC
  (if (not (Variables|Default|GetIsFire))
    (Variables|Default|SetIsFire true)
    (Audio|PlaySoundatLocation (Variables|Default|GetFireSound) (Transformation|GetWorldLocation (Variables|Default|GetItem_Mesh)) "0, 0, 0" 1.0 1.0 0.0 0 0 0 0)
    (Variables|/Game/BodycamFPSKIT/Blueprints/Components/AC_ProceduralAnimation.AC_ProceduralAnimation_C|SetLeftHandAlpha (Variables|/Game/BodycamFPSKIT/Blueprints/BP_FPCharacter.BP_FPCharacter_C|GetAC_ProceduralAnimation (Variables|Default|GetPlayerRef)) 1.0)
    (Default|PlayAnimation (Variables|/Game/BodycamFPSKIT/Blueprints/BP_FPCharacter.BP_FPCharacter_C|GetAC_ProceduralAnimation _playerref) (Variables|/Script/Engine.Character|GetMesh _playerref) (Utilities|Select :Index (Variables|Components|GetAnimationIndexToPlay) :Option%200 (Variables|Animations|GetAttack_1) :Option%201 (Variables|Animations|GetAttack_2)) 1 1.0 0.01 0.01 "arms")
    (Utilities|FlowControl|Sequence
      (:then_0
        (CallFunction|FireHitScan false (Variables|Default|GetRange) "NewEnumerator0" true false)
        (Math|Integer|IncrementInt (Variables|Components|GetAnimationIndexToPlay)
          (:%20%20
            (if (== (Variables|Components|GetAnimationIndexToPlay) 2)
              (Variables|Components|SetAnimationIndexToPlay 0)))))
      (:then_1
        (Utilities|FlowControl|Delay 0.2)
        (Variables|/Game/BodycamFPSKIT/Blueprints/Components/AC_ProceduralAnimation.AC_ProceduralAnimation_C|SetLeftHandAlpha (Variables|/Game/BodycamFPSKIT/Blueprints/BP_FPCharacter.BP_FPCharacter_C|GetAC_ProceduralAnimation (Variables|Default|GetPlayerRef)) 0.0)
        (Variables|Default|SetIsFire false)))))

(fn ConstructionScript
  (|CallParentFunction))