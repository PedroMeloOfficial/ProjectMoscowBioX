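; Base Blueprint for melee weapons in the Bodycam FPS kit, providing knife attack and inspect behavior.
; BeginFire alternates two arm attack animations through the player's ACProceduralAnimation, with sound, left-hand alpha override and an attached ribbon trail.
; A delayed melee hit-scan deals with the strike, and a timer based on animation length resets the attack state and trail.
; Inspect is blocked while reloading, inspecting, aiming or attacking.
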(event EventDestroyed
  (Variables|/Game/BodycamFPSKIT/Blueprints/Components/AC_ProceduralAnimation.AC_ProceduralAnimation_C|SetLeftHandAlpha (Variables|/Game/BodycamFPSKIT/Blueprints/BP_FPCharacter.BP_FPCharacter_C|GetAC_ProceduralAnimation (Variables|Default|GetPlayerRef)) 0.0)
  (bind _trailref (Variables|Default|GetTrailRef)
    (:then
      (Components|Activation|Deactivate _trailref))
    (:else)))

(event EventInspect
  (bind _playerref (Variables|Default|GetPlayerRef))
  ;[0 0 0] INSPECT
  (if (Math|Boolean|ANDBoolean (not (Variables|Default|GetReloading)) (not (Variables|Default|GetIsInspect)) (not (Variables|/Game/BodycamFPSKIT/Blueprints/BP_FPCharacter.BP_FPCharacter_C|GetIsAim (Variables|Default|GetPlayerRef))) (not (Variables|Default|GetIsFire)))
    (Variables|Default|SetIsInspect true)
    (bind _playlength (Default|PlayAnimation (Variables|/Game/BodycamFPSKIT/Blueprints/BP_FPCharacter.BP_FPCharacter_C|GetAC_ProceduralAnimation _playerref) (Variables|/Script/Engine.Character|GetMesh _playerref) "/Game/BodycamFPSKIT/Character/Animations/WeaponAnims/Knife/Anim_Character_Knife_Inspect.Anim_Character_Knife_Inspect" 1 1.0 0.25 0.25 "arms"))
    (Utilities|FlowControl|Delay _playlength)
    (Variables|Default|SetIsInspect false)))

(event EventParentBeginPlay
  (Components|Animation|PlayAnimation (Variables|Default|GetItem_Mesh) (Variables|Default|GetEmptyWeaponAnim) false))

(event EventBeginFire
  (bind _playerref (Variables|Default|GetPlayerRef))
  (bind _ac_proceduralanimation (Variables|/Game/BodycamFPSKIT/Blueprints/BP_FPCharacter.BP_FPCharacter_C|GetAC_ProceduralAnimation _playerref))
  ;[0 0 0] FIRE LOGIC
  (if (not (Variables|Default|GetIsFire))
    (Variables|Default|SetIsFire true)
    (Audio|PlaySoundatLocation (Variables|Default|GetFireSound) (Transformation|GetWorldLocation (Variables|Default|GetItem_Mesh)) "0, 0, 0" 1.0 1.0 0.0 0 0 0 0)
    (Variables|/Game/BodycamFPSKIT/Blueprints/Components/AC_ProceduralAnimation.AC_ProceduralAnimation_C|SetLeftHandAlpha _ac_proceduralanimation 1.0)
    (bind _playlength (Default|PlayAnimation _ac_proceduralanimation (Variables|/Script/Engine.Character|GetMesh _playerref) (Utilities|Select :Index (Variables|Components|GetAnimationIndexToPlay) :Option%200 (Variables|Animations|GetAttack_1) :Option%201 (Variables|Animations|GetAttack_2)) 1 1.0 0.05 0.05 "arms"))
    (Utilities|FlowControl|Sequence
      (:then_0
        (Math|Integer|IncrementInt (Variables|Components|GetAnimationIndexToPlay)
          (:%20%20
            (bind _returnvalue (Effects|SpawnEmitterAttached "/Game/BodycamFPSKIT/ParticleEffects/P_Knife_RibbonTrail.P_Knife_RibbonTrail" (Variables|Default|GetItem_Mesh) "knife" "0, 0, 0" "90.000000,0.000000,0.000000" "0.250000,0.250000,0.250000" "KeepRelativeOffset" true "AutoRelease"))
            (Variables|Default|SetTrailRef _returnvalue))))
      (:then_1
        (Utilities|FlowControl|Delay 0.3)
        (CallFunction|FireHitScan false (Variables|Default|GetRange) "NewEnumerator0" true false))
      (:then_2
        (Utilities|FlowControl|Delay (- _playlength 0.5))
        (Variables|/Game/BodycamFPSKIT/Blueprints/Components/AC_ProceduralAnimation.AC_ProceduralAnimation_C|SetLeftHandAlpha _ac_proceduralanimation 0.0)
        (Components|Activation|Deactivate (Variables|Default|GetTrailRef))
        (Variables|Default|SetIsFire false)
        (if (== (Variables|Components|GetAnimationIndexToPlay) 2)
          (Variables|Components|SetAnimationIndexToPlay 0))))))

(fn ConstructionScript
  (|CallParentFunction))