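; Base weapon item held by the player in the bodycam FPS kit, with empty Trigger, Reload, Inspect and Melee hooks.
; Timers drive single, burst and auto fire through Trigger, updating the player's procedural recoil and animation.
; FireHitScan traces from muzzle or camera for bullets, shotgun pellets and melee, handling damage, impact effects and decals.
; Helpers sync ammo with the player's item data and build a left-hand akimbo copy, recalculating ammo capacity.
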(event Custom|ParentBeginPlay
  ;[0 0 0] EVENTS
)

(event Custom|BeginFire
  (bind _weaponfirerate (Variables|ItemStats|GetWeaponFireRate))
  (bind _weaponfirerate_2 (Variables|ItemStats|GetWeaponFireRate))
  (bind _weaponfirerate_3 (Variables|ItemStats|GetWeaponFireRate))
  ;[0 0 0] FIRE LOGIC
  (if (not (<= (Variables|ItemStats|GetAmmoCount) 0))
    (if (not (Variables|Logical|GetIsFire))
      (if (and (Utilities|Enum|Equal(Enum) (Variables|ItemStats|GetReloadType) "NewEnumerator2") (Variables|Logical|GetReloading))
        (Variables|Logical|SetIsReloadStopped true)
        (elif (not (Variables|Logical|GetReloading))
          (Variables|Logical|SetIsFire true)
          (Variables|/Game/BodycamFPSKIT/Blueprints/Components/AC_ProceduralAnimation.AC_ProceduralAnimation_C|SetIsFire (Variables|/Game/BodycamFPSKIT/Blueprints/BP_FPCharacter.BP_FPCharacter_C|GetAC_ProceduralAnimation (Variables|Default|GetPlayerRef)) true)
          (switch Utilities|FlowControl|Switch|SwitchonENUM_FireMode (Variables|ItemStats|GetFireMode)
            (:NewEnumerator0
              (CallFunction|Trigger)
              (Utilities|FlowControl|Sequence
                (:then_0
                  (Utilities|FlowControl|Delay _weaponfirerate_2)
                  (Variables|Logical|SetIsFire false)
                  (Variables|/Game/BodycamFPSKIT/Blueprints/Components/AC_ProceduralAnimation.AC_ProceduralAnimation_C|SetIsFire (Variables|/Game/BodycamFPSKIT/Blueprints/BP_FPCharacter.BP_FPCharacter_C|GetAC_ProceduralAnimation (Variables|Default|GetPlayerRef)) false)
                  (Variables|Weapon|SetShakeNow (Variables|Weapon|GetCameraShakeDefault)))
                (:then_1
                  (Utilities|FlowControl|Delay (- _weaponfirerate_2 (Variables|Logical|GetSingleShotRecoilResetTime)))
                  (Default|ResetRecoil (Variables|/Game/BodycamFPSKIT/Blueprints/BP_FPCharacter.BP_FPCharacter_C|GetAC_ProceduralRecoil (Variables|Default|GetPlayerRef))))))
            (:NewEnumerator2
              (bind _returnvalue (Utilities|Time|SetTimerbyEvent (delegate Custom|BurstFire) _weaponfirerate_3 true true (* _weaponfirerate_3 -1.0))))
            (:NewEnumerator4
              (bind _returnvalue_2 (Utilities|Time|SetTimerbyEvent (delegate Custom|FinishFire) _weaponfirerate true true (* _weaponfirerate -1.0))))))))))

(event Custom|FinishFire
  ;[0 0 0] FIRE LOGIC
  (CallFunction|Trigger))

(event Custom|Trigger
  ;[0 0 0] EVENTS
)

(event Custom|Reload
  ;[0 0 0] EVENTS
)

(event Custom|ChangeFireMode
  ;[0 0 0] CHANGE FIRE MODE
  (Variables|Logical|SetSelectedFireMode (Math|Conversions|ToInteger(Byte) (Variables|ItemStats|GetFireMode)))
  (if (not (Variables|ItemStats|GetFireModNotChangable))
    (if (== (Variables|Logical|GetSelectedFireMode) 2)
      (Variables|Logical|SetSelectedFireMode 0)
      (else
        (Variables|Logical|SetSelectedFireMode (Math|Integer|Clamp(Integer) (+ (Variables|Logical|GetSelectedFireMode) 1) 0 2))))
    (Variables|ItemStats|SetFireMode (Utilities|Enum|ByteToEnumENUM_FireMode (Math|Conversions|ToByte(Integer) (Variables|Logical|GetSelectedFireMode))))))

(event Custom|SpawnAttachments
  ;[0 0 0] EVENTS
)

(event Custom|StopFire
  ;[0 0 0] FIRE LOGIC
  (Utilities|Time|ClearandInvalidateTimerbyHandle (stale Custom|BeginFire _returnvalue_2))
  (Default|ResetRecoil (Variables|/Game/BodycamFPSKIT/Blueprints/BP_FPCharacter.BP_FPCharacter_C|GetAC_ProceduralRecoil (Variables|Default|GetPlayerRef)))
  (Variables|Weapon|SetShakeNow (Variables|Weapon|GetCameraShakeDefault))
  (switch Utilities|FlowControl|Switch|SwitchonENUM_FireMode (Variables|ItemStats|GetFireMode)
    (:NewEnumerator4
      (Variables|Logical|SetIsFire false)
      (Variables|/Game/BodycamFPSKIT/Blueprints/Components/AC_ProceduralAnimation.AC_ProceduralAnimation_C|SetIsFire (Variables|/Game/BodycamFPSKIT/Blueprints/BP_FPCharacter.BP_FPCharacter_C|GetAC_ProceduralAnimation (Variables|Default|GetPlayerRef)) false))))

(event Custom|Inspect
  ;[0 0 0] EVENTS
)

(event Custom|BurstFire
  ;[0 0 0] FIRE LOGIC
  (bind _counter (Utilities|FlowControl|DoN 3 :!label _label)
    (:Exit
      (CallFunction|Trigger)
      (if (== _counter 3)
        (Utilities|Time|ClearandInvalidateTimerbyHandle (stale Custom|BeginFire _returnvalue))
        (Variables|Logical|SetIsFire false)
        (Variables|/Game/BodycamFPSKIT/Blueprints/Components/AC_ProceduralAnimation.AC_ProceduralAnimation_C|SetIsFire (Variables|/Game/BodycamFPSKIT/Blueprints/BP_FPCharacter.BP_FPCharacter_C|GetAC_ProceduralAnimation (Variables|Default|GetPlayerRef)) false)
        (Default|ResetRecoil (Variables|/Game/BodycamFPSKIT/Blueprints/BP_FPCharacter.BP_FPCharacter_C|GetAC_ProceduralRecoil (Variables|Default|GetPlayerRef)))
        (Variables|Weapon|SetShakeNow (Variables|Weapon|GetCameraShakeDefault))
        (goto _label Reset)))))

(event Custom|Melee
  ;[0 0 0] EVENTS
)

(event EventBeginPlay
  ;[0 0 0] SETUP ITEM ON HAND
  (bind _asbp_fpcharacter (Utilities|Casting|CastToBP_FPCharacter (Game|Player|GetPlayerPawn 0)))
  (Variables|Default|SetPlayerRef _asbp_fpcharacter)
  (Default|SocketOffset (Variables|Default|GetPlayerRef) (Variables|ItemStats|GetHand_R_SocketOffset))
  (CallFunction|ParentBeginPlay))

(fn ConstructionScript
  (Components|SkinnedMesh|SetSkinnedAssetandUpdate (Variables|Default|GetItem_Mesh) (Variables|Weapon|GetMesh) true)
  (Rendering|SetVisibility (Variables|Default|GetSpareMag) false false)
  ;[0 0 0] Attach Optic Sight To Slide Bone On The Weapon
  (Transformation|AttachComponentToComponent (Variables|Default|GetOpticSight) (Variables|Default|GetItem_Mesh) "slide" "KeepRelative" "KeepRelative" "KeepRelative" false)
  (if (!= (Variables|Weapon|GetSpareMagMesh) 0)
    (Components|StaticMesh|SetStaticMesh (Variables|Default|GetSpareMag) (Variables|Weapon|GetSpareMagMesh))
    (Transformation|AttachComponentToComponent (Variables|Default|GetSpareMag) (Variables|Default|GetItem_Mesh) (Variables|Weapon|GetSpareMagSocket) "SnapToTarget" "SnapToTarget" "SnapToTarget" false)))

(fn FireHitScan
  (params (DrawDebug :type Boolean) (Range :type Float%20%28double-precision%29) (TraceStyle :type ENUM_LineTraceStyles%20Enum :default "NewEnumerator7") (IsMelee :type Boolean) (IsShotgun :type Boolean) (RefMesh :type Scene%20Component%20Object%20Reference))
  (bind _returnvalue (Math|Random|RandomFloatinRange 0.0 3.6e+02))
  (bind _returnvalue_2 (Transformation|GetSocketRotation RefMesh "Muzzle"))
  (bind _returnvalue_3 (Transformation|GetSocketLocation RefMesh "Muzzle"))
  (bind _playerref (Variables|Default|GetPlayerRef))
  (bind _spread (Variables|ItemStats|GetSpread))
  (bind _spread_2 (Variables|ItemStats|GetSpread))
  (bind _playerref_2 (Variables|Default|GetPlayerRef))
  (bind _playerref_3 (Variables|Default|GetPlayerRef))
  (bind _playerref_4 (Variables|Default|GetPlayerRef))
  (bind _returnvalue_4 (Math|Vector|GetForwardVector _returnvalue_2))
  (bind _firstpersoncamera (Variables|/Game/BodycamFPSKIT/Blueprints/BP_FPCharacter.BP_FPCharacter_C|GetFirstPersonCamera _playerref))
  (bind _hud (Variables|/Game/BodycamFPSKIT/Blueprints/BP_FPCharacter.BP_FPCharacter_C|GetHUD _playerref_2))
  (bind _returnvalue_5 (Transformation|GetWorldLocation _firstpersoncamera))
  (bind _returnvalue_6 (Math|Random|RandomUnitVectorinConeinDegrees _returnvalue_4 _spread))
  (bind _returnvalue_7 (Math|Vector|GetForwardVector _firstpersoncamera))
  (bind _returnvalue_8 (* _returnvalue_6 Range))
  (bind _returnvalue_9 (Math|Random|RandomUnitVectorinConeinDegrees _returnvalue_7 _spread_2))
  (bind _returnvalue_10 (* _returnvalue_9 Range))
  (bind _returnvalue_11 (+ _returnvalue_3 _returnvalue_8))
  (bind (_x _y _z) (Math|Vector|BreakVector _returnvalue_11))
  (bind _returnvalue_12 (+ _returnvalue_5 _returnvalue_10))
  (bind (_x_2 _y_2 _z_2) (Math|Vector|BreakVector _returnvalue_12))
  (if IsShotgun
    (for _index (range 1 7)
      (switch Utilities|FlowControl|Switch|SwitchonENUM_LineTraceStyles TraceStyle
        (:NewEnumerator7
          ;[0 0 0] LINETRACE FROM MUZZLE
          (bind _outhit (Collision|LineTraceByChannel _returnvalue_3 (Math|Vector|SelectVector (Math|Vector|MakeVector _x (+ _y (Math|Random|RandomFloatinRange -3.5e+02 3.5e+02)) (+ _z (Math|Random|RandomFloatinRange -3.5e+02 3.5e+02))) _returnvalue_11 IsShotgun) "TraceTypeQuery2" false (Utilities|Array|MakeArray (Variables|Default|GetPlayerRef)) (select false "ForDuration" "None"))))
        (:NewEnumerator0
          ;[0 0 0] LINETRACE FROM CAMERA
          (bind _outhit_2 (Collision|LineTraceByChannel _returnvalue_5 (Math|Vector|SelectVector (Math|Vector|MakeVector _x_2 (+ _y_2 (Math|Random|RandomFloatinRange -3.5e+02 3.5e+02)) (+ _z_2 (Math|Random|RandomFloatinRange -3.5e+02 3.5e+02))) _returnvalue_12 IsShotgun) "TraceTypeQuery2" false (Utilities|Array|MakeArray (Variables|Default|GetPlayerRef)) (select false "ForDuration" "None")))))
      (LocalVariables|SetlocalHitTraceInfo (Utilities|Select :Index TraceStyle :NewEnumerator7 _outhit :NewEnumerator0 _outhit_2))
      (LocalVariables|SetIsHit (.bBlockingHit (Collision|BreakHitResult (Utilities|Select :Index TraceStyle :NewEnumerator7 _outhit :NewEnumerator0 _outhit_2))))
      (LocalVariables|SetImpactNormal (.ImpactNormal (Collision|BreakHitResult (Utilities|Select :Index TraceStyle :NewEnumerator7 _outhit :NewEnumerator0 _outhit_2))))
      (LocalVariables|SetImpactPoint (.ImpactPoint (Collision|BreakHitResult (Utilities|Select :Index TraceStyle :NewEnumerator7 _outhit :NewEnumerator0 _outhit_2))))
      (LocalVariables|SetHitComp (.HitComponent (Collision|BreakHitResult (Utilities|Select :Index TraceStyle :NewEnumerator7 _outhit :NewEnumerator0 _outhit_2))))
      (LocalVariables|SetBoneName (.HitBoneName (Collision|BreakHitResult (Utilities|Select :Index TraceStyle :NewEnumerator7 _outhit :NewEnumerator0 _outhit_2))))
      (LocalVariables|SetHitActor (.HitActor (Collision|BreakHitResult (Utilities|Select :Index TraceStyle :NewEnumerator7 _outhit :NewEnumerator0 _outhit_2))))
      (if IsMelee
        ;[0 0 0] MELEE IMPACT SOUND
        (if (LocalVariables|GetIsHit)
          (Audio|PlaySoundatLocation "/Game/BodycamFPSKIT/Audio/Character/Sound_Punch_Cue.Sound_Punch_Cue" (LocalVariables|GetImpactPoint) "0, 0, 0" 1.0 1.0 0.0 "/Game/BodycamFPSKIT/Audio/Attenuation/ProjectileImpact_att.ProjectileImpact_att" 0 0 0)
          ;[0 0 0] CAST TO ENEMY BP
          (bind _asbp_enemy (Utilities|Casting|CastToBP_Enemy (LocalVariables|GetHitActor) :!label _label)
            (:then
              (LocalVariables|SetEnemyRef _asbp_enemy)
              ;[0 0 0] ENEMY HIT BLOOD PARTICLE
              (Audio|PlaySoundatLocation "/Game/BodycamFPSKIT/Audio/Character/HitMarker.HitMarker" (LocalVariables|GetImpactPoint) "0, 0, 0" (Math|Random|RandomFloatinRange 1.15 1.25) (Math|Random|RandomFloatinRange 0.95 1.05) 0.0 0 0 0 0)
              (if (> (Variables|/Game/BodycamFPSKIT/Blueprints/Enemy/BP_Enemy.BP_Enemy_C|GetHealth (LocalVariables|GetEnemyRef)) 0.0)
                (Game|Damage|ApplyDamage (LocalVariables|GetEnemyRef) (Math|Float|SelectFloat 1e+02 25.0 (== (LocalVariables|GetBoneName) "head")) 0 0)
                (if (== (LocalVariables|GetBoneName) "head")
                  (Default|HitMarkerDead _hud)
                  (else
                    (Default|HitmarkerEffect _hud)))
                (Default|HitReaction (LocalVariables|GetEnemyRef) (LocalVariables|GetBoneName) (* (LocalVariables|GetImpactNormal) -5e+03))
                (Niagara|SpawnSystematLocation "/Game/BodycamFPSKIT/ParticleEffects/NS_Smoke_Blood_System.NS_Smoke_Blood_System" (LocalVariables|GetImpactPoint) (Math|Conversions|RotationFromXVector (LocalVariables|GetImpactNormal)) "1.000000,1.000000,1.000000" true true "AutoRelease")
                (else
                  (Audio|PlaySoundatLocation "/Game/BodycamFPSKIT/Audio/Character/Rifle_ImpactBody_Cue.Rifle_ImpactBody_Cue" (LocalVariables|GetImpactPoint) "0, 0, 0" 1.0 1.0 0.0 0 0 0 0))))
            (:CastFailed
              (bind _asmonster_nbc (Utilities|Casting|CastToMonster_NBC (LocalVariables|GetHitActor))
                (:then
                  (LocalVariables|SetMonsterRef _asmonster_nbc)
                  ;[0 0 0] ENEMY HIT BLOOD PARTICLE
                  (if (> (Variables|/Game/MonsterAi_Kit/Monster_NBC.Monster_NBC_C|GetHealth (LocalVariables|GetMonsterRef)) 0.0)
                    (Game|Damage|ApplyPointDamage (LocalVariables|GetMonsterRef) (Math|Float|SelectFloat 1e+02 (Variables|ItemStats|GetDamage) (== (LocalVariables|GetBoneName) "head")) (Transformation|GetActorLocation _playerref_4) (LocalVariables|GetlocalHitTraceInfo) 0 _playerref_4)
                    (else
                      (Audio|PlaySoundatLocation "/Game/BodycamFPSKIT/Audio/Character/Rifle_ImpactBody_Cue.Rifle_ImpactBody_Cue" (LocalVariables|GetImpactPoint) "0, 0, 0" 1.0 1.0 0.0 0 0 0 0))))
                (:CastFailed
                  (Utilities|FlowControl|Sequence
                    (:then_0
                      ;[0 0 0] IMPACT PARTICLE AND HIT EFFECTS
                      (bind _returnvalue_13 (Niagara|SpawnSystematLocation (Variables|Default|GetImpactSurfaceParticle) (LocalVariables|GetImpactPoint) (Math|Conversions|RotationFromXVector (LocalVariables|GetImpactNormal))))
                      (Transformation|SetWorldLocation _returnvalue_13 (LocalVariables|GetImpactPoint) false false)
                      (Class|NiagaraDataInterfaceArrayFunctionLibrary|SetNiagaraArrayPosition _returnvalue_13 "User.ImpactPositions" (Utilities|Array|MakeArray (LocalVariables|GetImpactPoint)))
                      (Class|NiagaraDataInterfaceArrayFunctionLibrary|SetNiagaraArrayVector _returnvalue_13 "User.ImpactNormals" (Utilities|Array|MakeArray (LocalVariables|GetImpactNormal)))
                      (Class|NiagaraComponent|SetVariableInt _returnvalue_13 "User.NumberOfHits" 1)
                      (Utilities|IsValid (LocalVariables|GetHitComp)
                        (:Is%20Valid
                          (if (Physics|IsSimulatingPhysics (LocalVariables|GetHitComp) "None")
                            (Physics|AddImpulseatLocation (LocalVariables|GetHitComp) (* (LocalVariables|GetImpactNormal) -5e+03) (LocalVariables|GetImpactPoint) (LocalVariables|GetBoneName))))))
                    (:then_1
                      ;[0 0 0] ENEMY SPAWNER (YOU CAN REMOVE THIS IF YOU DON'T WANT)
                      (bind _asbp_enemy_tester (Utilities|Casting|CastToBP_EnemyTester (LocalVariables|GetHitActor)))
                      (if (Utilities|Enum|Equal(Enum) (Utilities|GetDisplayName (LocalVariables|GetHitComp)) "BP_EnemyTester.Trigger Cube")
                        (Default|RespawnEnemies _asbp_enemy_tester)))))))))
        (else
          (if (Variables|Logical|GetIsSilenced)
            _
            (else
              (Class|Actor|MakeNoise 5.0 _playerref_3 (Transformation|GetActorLocation _playerref_3) 5e+03 "none")))
          (if (LocalVariables|GetIsHit)
            ;[0 0 0] FIRE TRACE AND IMPACT SOUND
            (Audio|PlaySoundatLocation "/Game/BodycamFPSKIT/Audio/Character/Rifle_ImpactSurface_Cue.Rifle_ImpactSurface_Cue" (LocalVariables|GetImpactPoint) "0, 0, 0" 0.3 1.0 0.0 "/Game/BodycamFPSKIT/Audio/Attenuation/ProjectileImpact_att.ProjectileImpact_att" 0 0 0))
          (Utilities|FlowControl|Sequence
            (:then_0
              (goto _label))
            (:then_1
              ;[0 0 0] SPAWN DECAL
              (bind _asskeletal_mesh_component (Utilities|Casting|CastToSkeletalMeshComponent (LocalVariables|GetHitComp))
                (:then
                  (bind _returnvalue_14 (Class|GameplayStatics|SpawnDecalAttached "/Game/BodycamFPSKIT/ParticleEffects/Materials/M_Blood_Decal.M_Blood_Decal" "4.000000,7.500000,7.500000" _asskeletal_mesh_component (LocalVariables|GetBoneName) (LocalVariables|GetImpactPoint) (Math|Rotator|MakeRotationfromAxes (.X (Math|Rotator|BreakRotIntoAxes (Math|Conversions|RotationFromXVector (LocalVariables|GetImpactNormal)))) (Math|Vector|RotateVectorAroundAxis (.Y (Math|Rotator|BreakRotIntoAxes (Math|Conversions|RotationFromXVector (LocalVariables|GetImpactNormal)))) _returnvalue (.X (Math|Rotator|BreakRotIntoAxes (Math|Conversions|RotationFromXVector (LocalVariables|GetImpactNormal))))) (Math|Vector|RotateVectorAroundAxis (.Z (Math|Rotator|BreakRotIntoAxes (Math|Conversions|RotationFromXVector (LocalVariables|GetImpactNormal)))) _returnvalue (.X (Math|Rotator|BreakRotIntoAxes (Math|Conversions|RotationFromXVector (LocalVariables|GetImpactNormal)))))) "KeepWorldPosition" 15.0))
                  (Utilities|IsValid _returnvalue_14
                    (:Is%20Valid
                      (Rendering|Components|Decal|SetFadeScreenSize _returnvalue_14 0.0))))
                (:CastFailed
                  (bind _returnvalue_15 (Class|GameplayStatics|SpawnDecalAttached "/Game/BodycamFPSKIT/ParticleEffects/Materials/M_Impact_Decal.M_Impact_Decal" "4.000000,8.500000,8.500000" (LocalVariables|GetHitComp) "None" (LocalVariables|GetImpactPoint) (Math|Rotator|MakeRotationfromAxes (.X (Math|Rotator|BreakRotIntoAxes (Math|Conversions|RotationFromXVector (LocalVariables|GetImpactNormal)))) (Math|Vector|RotateVectorAroundAxis (.Y (Math|Rotator|BreakRotIntoAxes (Math|Conversions|RotationFromXVector (LocalVariables|GetImpactNormal)))) _returnvalue (.X (Math|Rotator|BreakRotIntoAxes (Math|Conversions|RotationFromXVector (LocalVariables|GetImpactNormal))))) (Math|Vector|RotateVectorAroundAxis (.Z (Math|Rotator|BreakRotIntoAxes (Math|Conversions|RotationFromXVector (LocalVariables|GetImpactNormal)))) _returnvalue (.X (Math|Rotator|BreakRotIntoAxes (Math|Conversions|RotationFromXVector (LocalVariables|GetImpactNormal)))))) "KeepWorldPosition" 15.0))
                  (Utilities|IsValid _returnvalue_15
                    (:Is%20Valid
                      (Rendering|Components|Decal|SetFadeScreenSize _returnvalue_15 0.0))))))))))
    (else
      (switch Utilities|FlowControl|Switch|SwitchonENUM_LineTraceStyles TraceStyle
        (:NewEnumerator7
          (bind _outhit_3 (Collision|LineTraceByChannel _returnvalue_3 (Math|Vector|SelectVector (Math|Vector|MakeVector _x (+ _y (Math|Random|RandomFloatinRange -3.5e+02 3.5e+02)) (+ _z (Math|Random|RandomFloatinRange -3.5e+02 3.5e+02))) _returnvalue_11 IsShotgun) "TraceTypeQuery2" false (Utilities|Array|MakeArray (Variables|Default|GetPlayerRef)) (select false "ForDuration" "None"))))
        (:NewEnumerator0
          (bind _outhit_4 (Collision|LineTraceByChannel _returnvalue_5 (Math|Vector|SelectVector (Math|Vector|MakeVector _x_2 (+ _y_2 (Math|Random|RandomFloatinRange -3.5e+02 3.5e+02)) (+ _z_2 (Math|Random|RandomFloatinRange -3.5e+02 3.5e+02))) _returnvalue_12 IsShotgun) "TraceTypeQuery2" false (Utilities|Array|MakeArray (Variables|Default|GetPlayerRef)) (select false "ForDuration" "None")))))
      (LocalVariables|SetlocalHitTraceInfo (Utilities|Select :Index TraceStyle :NewEnumerator7 _outhit_3 :NewEnumerator0 _outhit_4))
      (LocalVariables|SetIsHit (.bBlockingHit (Collision|BreakHitResult (Utilities|Select :Index TraceStyle :NewEnumerator7 _outhit_3 :NewEnumerator0 _outhit_4))))
      (LocalVariables|SetImpactNormal (.ImpactNormal (Collision|BreakHitResult (Utilities|Select :Index TraceStyle :NewEnumerator7 _outhit_3 :NewEnumerator0 _outhit_4))))
      (LocalVariables|SetImpactPoint (.ImpactPoint (Collision|BreakHitResult (Utilities|Select :Index TraceStyle :NewEnumerator7 _outhit_3 :NewEnumerator0 _outhit_4))))
      (LocalVariables|SetHitComp (.HitComponent (Collision|BreakHitResult (Utilities|Select :Index TraceStyle :NewEnumerator7 _outhit_3 :NewEnumerator0 _outhit_4))))
      (LocalVariables|SetBoneName (.HitBoneName (Collision|BreakHitResult (Utilities|Select :Index TraceStyle :NewEnumerator7 _outhit_3 :NewEnumerator0 _outhit_4))))
      (LocalVariables|SetHitActor (.HitActor (Collision|BreakHitResult (Utilities|Select :Index TraceStyle :NewEnumerator7 _outhit_3 :NewEnumerator0 _outhit_4))))
      (if IsMelee
        (if (LocalVariables|GetIsHit)
          (Audio|PlaySoundatLocation "/Game/BodycamFPSKIT/Audio/Character/Sound_Punch_Cue.Sound_Punch_Cue" (LocalVariables|GetImpactPoint) "0, 0, 0" 1.0 1.0 0.0 "/Game/BodycamFPSKIT/Audio/Attenuation/ProjectileImpact_att.ProjectileImpact_att" 0 0 0)
          (bind _asbp_enemy_2 (Utilities|Casting|CastToBP_Enemy (LocalVariables|GetHitActor) :!label _label_2)
            (:then
              (LocalVariables|SetEnemyRef _asbp_enemy_2)
              (Audio|PlaySoundatLocation "/Game/BodycamFPSKIT/Audio/Character/HitMarker.HitMarker" (LocalVariables|GetImpactPoint) "0, 0, 0" (Math|Random|RandomFloatinRange 1.15 1.25) (Math|Random|RandomFloatinRange 0.95 1.05) 0.0 0 0 0 0)
              (if (> (Variables|/Game/BodycamFPSKIT/Blueprints/Enemy/BP_Enemy.BP_Enemy_C|GetHealth (LocalVariables|GetEnemyRef)) 0.0)
                (Game|Damage|ApplyDamage (LocalVariables|GetEnemyRef) (Math|Float|SelectFloat 1e+02 25.0 (== (LocalVariables|GetBoneName) "head")) 0 0)
                (if (== (LocalVariables|GetBoneName) "head")
                  (Default|HitMarkerDead _hud)
                  (else
                    (Default|HitmarkerEffect _hud)))
                (Default|HitReaction (LocalVariables|GetEnemyRef) (LocalVariables|GetBoneName) (* (LocalVariables|GetImpactNormal) -5e+03))
                (Niagara|SpawnSystematLocation "/Game/BodycamFPSKIT/ParticleEffects/NS_Smoke_Blood_System.NS_Smoke_Blood_System" (LocalVariables|GetImpactPoint) (Math|Conversions|RotationFromXVector (LocalVariables|GetImpactNormal)) "1.000000,1.000000,1.000000" true true "AutoRelease")
                (else
                  (Audio|PlaySoundatLocation "/Game/BodycamFPSKIT/Audio/Character/Rifle_ImpactBody_Cue.Rifle_ImpactBody_Cue" (LocalVariables|GetImpactPoint) "0, 0, 0" 1.0 1.0 0.0 0 0 0 0))))
            (:CastFailed
              (bind _asmonster_nbc_2 (Utilities|Casting|CastToMonster_NBC (LocalVariables|GetHitActor))
                (:then
                  (LocalVariables|SetMonsterRef _asmonster_nbc_2)
                  (if (> (Variables|/Game/MonsterAi_Kit/Monster_NBC.Monster_NBC_C|GetHealth (LocalVariables|GetMonsterRef)) 0.0)
                    (Game|Damage|ApplyPointDamage (LocalVariables|GetMonsterRef) (Math|Float|SelectFloat 1e+02 (Variables|ItemStats|GetDamage) (== (LocalVariables|GetBoneName) "head")) (Transformation|GetActorLocation _playerref_4) (LocalVariables|GetlocalHitTraceInfo) 0 _playerref_4)
                    (else
                      (Audio|PlaySoundatLocation "/Game/BodycamFPSKIT/Audio/Character/Rifle_ImpactBody_Cue.Rifle_ImpactBody_Cue" (LocalVariables|GetImpactPoint) "0, 0, 0" 1.0 1.0 0.0 0 0 0 0))))
                (:CastFailed
                  (Utilities|FlowControl|Sequence
                    (:then_0
                      (bind _returnvalue_16 (Niagara|SpawnSystematLocation (Variables|Default|GetImpactSurfaceParticle) (LocalVariables|GetImpactPoint) (Math|Conversions|RotationFromXVector (LocalVariables|GetImpactNormal))))
                      (Transformation|SetWorldLocation _returnvalue_16 (LocalVariables|GetImpactPoint) false false)
                      (Class|NiagaraDataInterfaceArrayFunctionLibrary|SetNiagaraArrayPosition _returnvalue_16 "User.ImpactPositions" (Utilities|Array|MakeArray (LocalVariables|GetImpactPoint)))
                      (Class|NiagaraDataInterfaceArrayFunctionLibrary|SetNiagaraArrayVector _returnvalue_16 "User.ImpactNormals" (Utilities|Array|MakeArray (LocalVariables|GetImpactNormal)))
                      (Class|NiagaraComponent|SetVariableInt _returnvalue_16 "User.NumberOfHits" 1)
                      (Utilities|IsValid (LocalVariables|GetHitComp)
                        (:Is%20Valid
                          (if (Physics|IsSimulatingPhysics (LocalVariables|GetHitComp) "None")
                            (Physics|AddImpulseatLocation (LocalVariables|GetHitComp) (* (LocalVariables|GetImpactNormal) -5e+03) (LocalVariables|GetImpactPoint) (LocalVariables|GetBoneName))))))
                    (:then_1
                      (bind _asbp_enemy_tester_2 (Utilities|Casting|CastToBP_EnemyTester (LocalVariables|GetHitActor)))
                      (if (Utilities|Enum|Equal(Enum) (Utilities|GetDisplayName (LocalVariables|GetHitComp)) "BP_EnemyTester.Trigger Cube")
                        (Default|RespawnEnemies _asbp_enemy_tester_2)))))))))
        (else
          (if (Variables|Logical|GetIsSilenced)
            _
            (else
              (Class|Actor|MakeNoise 5.0 _playerref_3 (Transformation|GetActorLocation _playerref_3) 5e+03 "none")))
          (if (LocalVariables|GetIsHit)
            (Audio|PlaySoundatLocation "/Game/BodycamFPSKIT/Audio/Character/Rifle_ImpactSurface_Cue.Rifle_ImpactSurface_Cue" (LocalVariables|GetImpactPoint) "0, 0, 0" 0.3 1.0 0.0 "/Game/BodycamFPSKIT/Audio/Attenuation/ProjectileImpact_att.ProjectileImpact_att" 0 0 0))
          (Utilities|FlowControl|Sequence
            (:then_0
              (goto _label_2))
            (:then_1
              (bind _asskeletal_mesh_component_2 (Utilities|Casting|CastToSkeletalMeshComponent (LocalVariables|GetHitComp))
                (:then
                  (bind _returnvalue_17 (Class|GameplayStatics|SpawnDecalAttached "/Game/BodycamFPSKIT/ParticleEffects/Materials/M_Blood_Decal.M_Blood_Decal" "4.000000,7.500000,7.500000" _asskeletal_mesh_component_2 (LocalVariables|GetBoneName) (LocalVariables|GetImpactPoint) (Math|Rotator|MakeRotationfromAxes (.X (Math|Rotator|BreakRotIntoAxes (Math|Conversions|RotationFromXVector (LocalVariables|GetImpactNormal)))) (Math|Vector|RotateVectorAroundAxis (.Y (Math|Rotator|BreakRotIntoAxes (Math|Conversions|RotationFromXVector (LocalVariables|GetImpactNormal)))) _returnvalue (.X (Math|Rotator|BreakRotIntoAxes (Math|Conversions|RotationFromXVector (LocalVariables|GetImpactNormal))))) (Math|Vector|RotateVectorAroundAxis (.Z (Math|Rotator|BreakRotIntoAxes (Math|Conversions|RotationFromXVector (LocalVariables|GetImpactNormal)))) _returnvalue (.X (Math|Rotator|BreakRotIntoAxes (Math|Conversions|RotationFromXVector (LocalVariables|GetImpactNormal)))))) "KeepWorldPosition" 15.0))
                  (Utilities|IsValid _returnvalue_17
                    (:Is%20Valid
                      (Rendering|Components|Decal|SetFadeScreenSize _returnvalue_17 0.0))))
                (:CastFailed
                  (bind _returnvalue_18 (Class|GameplayStatics|SpawnDecalAttached "/Game/BodycamFPSKIT/ParticleEffects/Materials/M_Impact_Decal.M_Impact_Decal" "4.000000,8.500000,8.500000" (LocalVariables|GetHitComp) "None" (LocalVariables|GetImpactPoint) (Math|Rotator|MakeRotationfromAxes (.X (Math|Rotator|BreakRotIntoAxes (Math|Conversions|RotationFromXVector (LocalVariables|GetImpactNormal)))) (Math|Vector|RotateVectorAroundAxis (.Y (Math|Rotator|BreakRotIntoAxes (Math|Conversions|RotationFromXVector (LocalVariables|GetImpactNormal)))) _returnvalue (.X (Math|Rotator|BreakRotIntoAxes (Math|Conversions|RotationFromXVector (LocalVariables|GetImpactNormal))))) (Math|Vector|RotateVectorAroundAxis (.Z (Math|Rotator|BreakRotIntoAxes (Math|Conversions|RotationFromXVector (LocalVariables|GetImpactNormal)))) _returnvalue (.X (Math|Rotator|BreakRotIntoAxes (Math|Conversions|RotationFromXVector (LocalVariables|GetImpactNormal)))))) "KeepWorldPosition" 15.0))
                  (Utilities|IsValid _returnvalue_18
                    (:Is%20Valid
                      (Rendering|Components|Decal|SetFadeScreenSize _returnvalue_18 0.0))))))))))))

(fn SetWeaponAmmoData
  (params (IsPickUp :type Boolean))
  (if IsPickUp
    ;[0 0 0] ADD AMMO TO SLOT
    (switch Utilities|FlowControl|Switch|SwitchonENUM_ItemSlots (Variables|/Game/BodycamFPSKIT/Blueprints/BP_FPCharacter.BP_FPCharacter_C|GetEquippedWeapon (Variables|Default|GetPlayerRef))
      (:NewEnumerator0
        (bind _primaryslot (Variables|/Game/BodycamFPSKIT/Blueprints/BP_FPCharacter.BP_FPCharacter_C|GetPrimarySlot (Variables|Default|GetPlayerRef))
          (:then
            (Variables|ItemStats|SetAmmoCount (.AmmoCount (Utilities|Struct|BreakST_Item (Variables|/Game/BodycamFPSKIT/Blueprints/Interactables/DT_Item.DT_Item_C|GetItemData _primaryslot))))
            (Variables|ItemStats|SetMaxAmmo (.MaxAmmo (Utilities|Struct|BreakST_Item (Variables|/Game/BodycamFPSKIT/Blueprints/Interactables/DT_Item.DT_Item_C|GetItemData _primaryslot)))))
          (:else)))
      (:NewEnumerator10
        (bind _secondaryslot (Variables|/Game/BodycamFPSKIT/Blueprints/BP_FPCharacter.BP_FPCharacter_C|GetSecondarySlot (Variables|Default|GetPlayerRef))
          (:then
            (Variables|ItemStats|SetAmmoCount (.AmmoCount (Utilities|Struct|BreakST_Item (Variables|/Game/BodycamFPSKIT/Blueprints/Interactables/DT_Item.DT_Item_C|GetItemData _secondaryslot))))
            (Variables|ItemStats|SetMaxAmmo (.MaxAmmo (Utilities|Struct|BreakST_Item (Variables|/Game/BodycamFPSKIT/Blueprints/Interactables/DT_Item.DT_Item_C|GetItemData _secondaryslot)))))
          (:else)))
      (:NewEnumerator8
        (bind _throwableslot (Variables|/Game/BodycamFPSKIT/Blueprints/BP_FPCharacter.BP_FPCharacter_C|GetThrowableSlot (Variables|Default|GetPlayerRef))
          (:then
            (Variables|ItemStats|SetAmmoCount (.AmmoCount (Utilities|Struct|BreakST_Item (Variables|/Game/BodycamFPSKIT/Blueprints/Interactables/DT_Item.DT_Item_C|GetItemData _throwableslot))))
            (Variables|ItemStats|SetMaxAmmo (.MaxAmmo (Utilities|Struct|BreakST_Item (Variables|/Game/BodycamFPSKIT/Blueprints/Interactables/DT_Item.DT_Item_C|GetItemData _throwableslot)))))
          (:else))))
    (else
      ;[0 0 0] SET WEAPON AMMO DATA
      (bind _spawneditemref (Variables|/Game/BodycamFPSKIT/Blueprints/BP_FPCharacter.BP_FPCharacter_C|GetSpawnedItemRef (Variables|Default|GetPlayerRef))
        (:then
          (Variables|/Game/BodycamFPSKIT/Blueprints/Interactables/DT_Item.DT_Item_C|SetItemData _spawneditemref (Utilities|Struct|MakeST_Item (.WeaponData (Utilities|Struct|BreakST_Item (Variables|/Game/BodycamFPSKIT/Blueprints/Interactables/DT_Item.DT_Item_C|GetItemData _spawneditemref))) (Variables|ItemStats|GetAmmoCount) (Variables|ItemStats|GetMaxAmmo) (.Attachments (Utilities|Struct|BreakST_Item (Variables|/Game/BodycamFPSKIT/Blueprints/Interactables/DT_Item.DT_Item_C|GetItemData _spawneditemref))))))
        (:else)))))

(fn SetAmmo
  (params (AmmoCount :type Integer) (MaxAmmo :type Integer))
  (Variables|ItemStats|SetMaxAmmo MaxAmmo)
  (Variables|ItemStats|SetAmmoCount AmmoCount))

(fn AkimboSpawner
  (params (ReCalculateAmmo :type Boolean))
  (bind _weaponcapacity (Variables|ItemStats|GetWeaponCapacity))
  (bind _weaponcapacity_2 (Variables|ItemStats|GetWeaponCapacity))
  (bind _playerref (Variables|Default|GetPlayerRef))
  (bind _muzzle (Variables|Default|GetMuzzle))
  (bind _hand_l_socketoffset (Variables|ItemStats|GetHand_L_SocketOffset))
  (bind _opticsight (Variables|Default|GetOpticSight))
  (bind _laser (Variables|Default|GetLaser))
  (bind _returnvalue (Transformation|GetRelativeTransform _opticsight))
  (bind _returnvalue_2 (Transformation|GetRelativeTransform _muzzle))
  (bind _returnvalue_3 (Transformation|GetRelativeTransform _laser))
  (bind _returnvalue_4 (* _weaponcapacity_2 2))
  (bind _spawneditemref (Variables|/Game/BodycamFPSKIT/Blueprints/BP_FPCharacter.BP_FPCharacter_C|GetSpawnedItemRef _playerref))
  (bind _itemdata (Variables|/Game/BodycamFPSKIT/Blueprints/Interactables/DT_Item.DT_Item_C|GetItemData _spawneditemref))
  (bind (_ammocount _maxammo) (Utilities|Struct|BreakST_Item _itemdata))
  (bind _returnvalue_5 (+ _ammocount _maxammo))
  (bind _returnvalue_6 (+ _ammocount _maxammo))
  (bind _returnvalue_7 (<= _returnvalue_6 _weaponcapacity))
  (bind _returnvalue_8 (<= _returnvalue_5 _returnvalue_4))
  (bind _returnvalue_9 (Math|Integer|SelectInt _returnvalue_5 _returnvalue_4 _returnvalue_8))
  (bind _returnvalue_10 (Math|Integer|SelectInt _returnvalue_6 _weaponcapacity _returnvalue_7))
  (if (Utilities|Enum|Equal(Enum) (Utilities|Struct|BreakST_Attachments (Utilities|Struct|BreakST_Item (Variables|/Game/BodycamFPSKIT/Blueprints/Interactables/DT_Item.DT_Item_C|GetItemData (Variables|/Game/BodycamFPSKIT/Blueprints/BP_FPCharacter.BP_FPCharacter_C|GetSpawnedItemRef (Variables|Default|GetPlayerRef))))) "NewEnumerator4")
    (Utilities|FlowControl|Sequence
      (:then_0
        (Variables|Components|GetAkimboMesh
          (:then)
          (:else
            (bind _returnvalue_11 (AddComponent|AddSkeletalMeshComponent false))
            (bind _output_get (Variables|Components|SetAkimboMesh _returnvalue_11))
            (Components|SkeletalMesh|SetSkeletalMeshAsset _output_get (Variables|Weapon|GetMesh))
            (Transformation|AttachComponentToComponent _output_get (Variables|/Script/Engine.Character|GetMesh (Variables|Default|GetPlayerRef)) "hand_l" "SnapToTarget" "SnapToTarget" "SnapToTarget" true)
            (Transformation|AddLocalOffset (Variables|Components|GetAkimboMesh) (.location _hand_l_socketoffset) false false)
            (Transformation|AddLocalRotation (Variables|Components|GetAkimboMesh) (.rotation _hand_l_socketoffset) false false)
            (bind _returnvalue_12 (AddComponent|AddStaticMeshComponent false))
            (bind _output_get_2 (Variables|Components|SetAkimboMuzzle _returnvalue_12))
            (Transformation|AttachComponentToComponent _output_get_2 (Variables|Components|GetAkimboMesh) "" "SnapToTarget" "SnapToTarget" "SnapToTarget" true)
            (Transformation|AddLocalOffset _output_get_2 (.location _returnvalue_2) false false)
            (Transformation|SetRelativeRotation _output_get_2 (.rotation _returnvalue_2) false false)
            (bind _returnvalue_13 (AddComponent|AddStaticMeshComponent false))
            (bind _output_get_3 (Variables|Components|SetAkimboLaser _returnvalue_13))
            (Transformation|AttachComponentToComponent _output_get_3 (Variables|Components|GetAkimboMesh) "" "SnapToTarget" "SnapToTarget" "SnapToTarget" true)
            (Transformation|AddLocalOffset _output_get_3 (.location _returnvalue_3) false false)
            (Transformation|SetRelativeRotation _output_get_3 (.rotation _returnvalue_3) false false)
            (bind _returnvalue_14 (AddComponent|AddStaticMeshComponent false))
            (bind _output_get_4 (Variables|Components|SetAkimboSight _returnvalue_14))
            (Transformation|AttachComponentToComponent _output_get_4 (Variables|Components|GetAkimboMesh) "Slide" "KeepRelative" "KeepRelative" "SnapToTarget" true)
            (Transformation|AddLocalOffset _output_get_4 (.location _returnvalue) false false)
            (Transformation|SetRelativeRotation _output_get_4 (.rotation _returnvalue) false false))))
      (:then_1
        (if ReCalculateAmmo
          (CallFunction|SetAmmo _returnvalue_9 (Math|Integer|Clamp(Integer) (- _returnvalue_5 _returnvalue_9) 0 999999))
          (CallFunction|SetWeaponAmmoData false))))
    (elif ReCalculateAmmo
      (CallFunction|SetAmmo _returnvalue_10 (Math|Integer|Clamp(Integer) (- _returnvalue_6 _returnvalue_10) 0 999999))
      (CallFunction|SetWeaponAmmoData false))))