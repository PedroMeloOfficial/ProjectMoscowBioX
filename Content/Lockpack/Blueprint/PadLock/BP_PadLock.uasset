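; Multiplayer combination padlock puzzle that hides itself, opens its target door and is destroyed once the password is entered.
; Inputs select a wheel, highlighted through dynamic material glow, and turn it in 36-degree digit steps via the padlock AnimBP.
; The password is checked locally against wheel angles.
; Server-to-multicast events replicate rotations, resets and the opening montage, while parent class calls handle puzzle entry and exit.
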(event Custom|Server_PasswordIsCorrect
  ;[0 0.7563 1] Password is correct
  (CallFunction|MulticastPasswordIsCorrect)
  (Collision|SetCollisionEnabled (Variables|Default|GetSphere) "NoCollision"))

(event Custom|Server_SetWheelRotation
  (params (WheelNumber :type Integer) (Rotation :type Float%20%28single-precision%29))
  ;[0 0.7563 1] Set wheel Rotation for all players
  (CallFunction|MulticastSetWheelRotation WheelNumber Rotation))

(event Custom|Multicast_PasswordIsCorrect
  ;[0 0.7563 1] Multicast Open safe lock door
  (Utilities|FlowControl|Delay 0.2)
  (Animation|Montage|PlayMontage (Variables|Default|GetSkeletalMesh) "/Game/Lockpack/Animation/AM_Padlock_open.AM_Padlock_open"
    (:then
      (Audio|PlaySoundatLocation (Variables|Sound|GetOpenSound) (Transformation|GetActorLocation) "0, 0, 0" 1.0 1.0 0.0 0 0 0))
    (:OnCompleted
      (CallFunction|MulticastOpenTargetDoor 0.0)
      (Rendering|SetActorHiddenInGame true)
      (Networking|SwitchHasAuthority
        (:Authority
          (Actor|DestroyActor))))))

(event Custom|Multicast_SetWheelRotation
  (params (WheelNumber :type Integer) (Rotation :type Float%20%28single-precision%29))
  ;[0 0.7563 1] Set wheel Rotation for all players
  (Default|SetWheelRotation (Variables|Ref|GetABPPadlockRef) WheelNumber Rotation))

(event Custom|Server_ResetLock
  ;[0 0.7563 1] Restart lock for all players
  (CallFunction|MulticastResetLock))

(event Custom|Multicast_ResetLock
  ;[0 0.7563 1] Restart lock for all players
  (CallFunction|ResetLock))

(event EventBeginPlay
  (bind _password (Variables|Password|GetPassword))
  (bind _returnvalue (Utilities|Array|Length _password))
  ;[1 1 1] Override begin play
  (|CallParentFunction)
  (bind _asabp_padlock (Utilities|Casting|CastToABP_Padlock (Components|SkeletalMesh|GetAnimInstance (Variables|Default|GetSkeletalMesh)))
    (:then
      (Variables|Ref|SetABPPadlockRef _asabp_padlock))
    (:CastFailed
      _))
  (Variables|Password|SetPasswordLength _returnvalue)
  (Utilities|Array|SetArrayElem (Variables|Password|GetWheelRotations) _returnvalue 0.0 true)
  (CallFunction|CreateDynamicMaterial))

(event EventClientEnterPuzzle
  (params (Character :type Character%20Object%20Reference))
  ;[0.01096 0.1119 0.1356] On entering puzzle, After call parent version, set show wheel to first one
  (|CallParentFunction Character)
  (CallFunction|SetShowWheel 0 true))

(event Input|ActionEvents|InputActionUp
  (params (Key :type Key%20Structure :default "None"))
  ;[0.1692 1 0.1706] Comment
  (:Pressed
    (Variables|Password|SetLastSelected%20Wheel (Variables|Password|GetSelectedWheel))
    (bind _result (Math|Integer|DecrementInt (Variables|Password|GetSelectedWheel))
      (:%20%20
        (if (< _result 0)
          (Variables|Password|SetSelectedWheel 0))
        (CallFunction|SetShowWheel (Variables|Password|GetLastSelected%20Wheel) false)
        (CallFunction|SetShowWheel (Variables|Password|GetSelectedWheel) true)
        (Audio|PlaySound2D (Variables|Sound|GetRollSound) 1.0 1.0 0.0 0 0)))))

(event Input|ActionEvents|InputActionDown
  (params (Key :type Key%20Structure :default "None"))
  ;[0.1692 1 0.1706] Comment
  (:Pressed
    (Variables|Password|SetLastSelected%20Wheel (Variables|Password|GetSelectedWheel))
    (bind _result (Math|Integer|IncrementInt (Variables|Password|GetSelectedWheel))
      (:%20%20
        (if (>= _result (Variables|Password|GetPasswordLength))
          (Variables|Password|SetSelectedWheel (- (Variables|Password|GetPasswordLength) 1)))
        (CallFunction|SetShowWheel (Variables|Password|GetLastSelected%20Wheel) false)
        (CallFunction|SetShowWheel (Variables|Password|GetSelectedWheel) true)
        (Audio|PlaySound2D (Variables|Sound|GetRollSound) 1.0 1.0 0.0 0 0)))))

(event Input|ActionEvents|InputActionRight
  (params (Key :type Key%20Structure :default "None"))
  ;[0.1692 1 0.1706] Rotate wheel to the right
  (:Pressed
    (Audio|PlaySound2D (Variables|Sound|GetSwitchSound) 1.0 1.0 0.0 0 0)
    (CallFunction|TurnWheel false)))

(event Input|ActionEvents|InputActionLeft
  (params (Key :type Key%20Structure :default "None"))
  ;[0.1692 1 0.1706] RotateWheel to the left
  (:Pressed
    (Audio|PlaySound2D (Variables|Sound|GetSwitchSound) 1.0 1.0 0.0 0 0)
    (CallFunction|TurnWheel true)))

(event Input|ActionEvents|InputActionAcceptKey
  (params (Key :type Key%20Structure :default "None"))
  ;[0.1692 1 0.1706] Check if password is correct
  (:Pressed
    (CallFunction|CheckPassword)))

(event Input|ActionEvents|InputActionInteract
  (params (Key :type Key%20Structure :default "None"))
  ;[0.1692 1 0.1706] Exit puzzle
  (:Pressed
    (CallFunction|ExitPuzzle)))

(event Input|ActionEvents|InputActionReset
  (params (Key :type Key%20Structure :default "None"))
  ;[0.1692 1 0.1706] ResetLock
  (:Pressed
    (CallFunction|ResetLock)
    (CallFunction|ServerResetLock)
    (Audio|PlaySound2D (Variables|Sound|GetResetSound) 1.0 1.0 0.0 0 0)))

(fn ConstructionScript
  (|CallParentFunction))

(fn TurnWheel
  (params (Clockwise? :type Boolean))
  ;[1 1 1] Change the wheel by 6degree then password proccess
  (bind _output_get (LocalVariables|SetTempRotation (+ (Utilities|Array|Get(acopy) (Variables|Password|GetWheelRotations) (Variables|Password|GetSelectedWheel)) (Math|Float|SelectFloat -36.0 36.0 Clockwise?))))
  (Utilities|Array|SetArrayElem (Variables|Password|GetWheelRotations) (Variables|Password|GetSelectedWheel) _output_get true)
  (Default|SetWheelRotation (Variables|Ref|GetABPPadlockRef) (Variables|Password|GetSelectedWheel) (LocalVariables|GetTempRotation))
  (CallFunction|ServerSetWheelRotation (Variables|Password|GetSelectedWheel) (LocalVariables|GetTempRotation)))

(fn CheckPassword
  ;[1 1 1] Compare each digit with correct digit to check if password is correct
  (bind (_array_element _array_index) (Utilities|Array|ForEachLoopwithBreak (Variables|Password|GetPassword) :!label _label)
    (:LoopBody
      (if (not (== _array_element (Math|Float|Truncate (/ (Class|KismetMathLibrary|ClampAxis (Utilities|Array|Get(acopy) (Variables|Password|GetWheelRotations) _array_index)) 36.0))))
        (LocalVariables|SetbPasswordIsCorrect false)
        (goto _label Break)))
    (:Completed
      ;[1 1 1] Open the door if it was correct
      (if (LocalVariables|GetbPasswordIsCorrect)
        (CallFunction|ServerPasswordIsCorrect)
        (CallFunction|ExitPuzzle)
        (else
          (Audio|PlaySound2D (Variables|Sound|GetInvalidSound) 1.0 1.0 0.0 0 0))))))

(fn CreateDynamicMaterial
  (for _index (range 0 (Variables|Password|GetPasswordLength))
    (bind _returnvalue (Rendering|Material|CreateDynamicMaterialInstance (Variables|Default|GetSkeletalMesh) _index (Utilities|Array|Get(acopy) (Rendering|Material|GetMaterials (Variables|Default|GetSkeletalMesh)) _index) "None" :!class /Script/Engine.PrimitiveComponent))
    (Utilities|Array|SetArrayElem (Variables|Materials|GetWheelsMaterial) _index _returnvalue true)))

(fn SetShowWheel
  (params (wheelIndex :type Integer) (Show :type Boolean))
  (Rendering|Material|SetScalarParameterValue (Utilities|Array|Get(acopy) (Variables|Materials|GetWheelsMaterial) wheelIndex) "Glowing Strength" (select Show (Variables|Materials|GetGlowing%20Strength) 0.0) :!class /Script/Engine.MaterialInstanceDynamic))

(fn ExitPuzzle
  (|CallParentFunction)
  (CallFunction|SetShowWheel (Variables|Password|GetSelectedWheel) false)
  (Variables|Password|SetSelectedWheel 0)
  (CallFunction|ResetLock))

(fn ResetLock
  (for (_ _array_index) (Variables|Password|GetWheelRotations)
    (Utilities|Array|SetArrayElem (Variables|Password|GetWheelRotations) _array_index 0.0)
    (Default|SetWheelRotation (Variables|Ref|GetABPPadlockRef) _array_index 0.0)))