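; BP_Clock is a multiplayer clock lock puzzle where players turn the hands to a target time to open a door.
; Construction encodes start and password times as minutes on a 12-hour dial, and CheckPassword wraps the current code modulo 720 to compare.
; Held left/right input steps one minute on a repeating timer, driving hand rotation through ABP_clock.
; Server-to-multicast events share rotation, resets and door opening, while the parent class handles exiting.
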(event Custom|Server_PasswordIsCorrect
  ;[0 0.7563 1] Password is correct
  (CallFunction|MulticastOpenTargetDoor 2.0)
  (Collision|SetCollisionEnabled (Variables|Default|GetSphere) "NoCollision"))

(event Custom|Server_SetWheelRotation
  (params (InPassword :type Integer))
  ;[0 0.7563 1] Set wheel Rotation for all players
  (CallFunction|MulticastSetWheelRotation InPassword))

(event Custom|Multicast_SetWheelRotation
  (params (InPassword :type Integer))
  ;[0 0.7563 1] Set wheel Rotation for all players
  (Default|SetHandsRotation (Variables|Refs|GetABP_ClockRef) InPassword))

(event Custom|Server_ResetLock
  ;[0 0.7563 1] Restart lock for all players
  (CallFunction|MulticastResetLock))

(event Custom|Multicast_ResetLock
  ;[0 0.7563 1] Restart lock for all players
  (CallFunction|ResetLock))

(event Custom|CheckAKey
  ;[0.1692 1 0.1706] Rotate wheel to the left
  (if (Variables|Input|GetAKey)
    (CallFunction|TurnHand true)
    (Utilities|Time|SetTimerbyEvent (delegate Custom|CheckAKey) 0.05)))

(event Custom|CheckDkey
  ;[0.1692 1 0.1706] Rotate wheel to the right
  (if (Variables|Input|GetDKey)
    (CallFunction|TurnHand false)
    (Utilities|Time|SetTimerbyEvent (delegate Custom|CheckDkey) 0.05)))

(event EventBeginPlay
  ;[1 1 1] Override begin play
  (|CallParentFunction)
  (bind _asabp_clock (Utilities|Casting|CastToABP_clock (Components|SkeletalMesh|GetAnimInstance (Variables|Default|GetSkeletalMesh))))
  (bind _output_get (Variables|Refs|SetABP_ClockRef _asabp_clock))
  (Default|SetHandsRotation _output_get (Variables|Password|GetStartCode))
  (Variables|Password|SetCurrentCode (Variables|Password|GetStartCode)))

(event Input|ActionEvents|InputActionReset
  (params (Key :type Key%20Structure :default "None"))
  ;[0.1692 1 0.1706] ResetLock
  (:Pressed
    (CallFunction|ResetLock)
    (CallFunction|ServerResetLock)))

(event Input|ActionEvents|InputActionInteract
  (params (Key :type Key%20Structure :default "None"))
  ;[0.1692 1 0.1706] Exit puzzle
  (:Pressed
    (CallFunction|ExitPuzzle)))

(event Input|ActionEvents|InputActionAcceptKey
  (params (Key :type Key%20Structure :default "None"))
  ;[0.1692 1 0.1706] Check if password is correct
  (:Pressed
    (CallFunction|CheckPassword)))

(event Input|ActionEvents|InputActionLeft
  (params (Key :type Key%20Structure :default "None"))
  ;[0.1692 1 0.1706] Rotate wheel to the left
  (:Pressed
    (Variables|Input|SetAKey true)
    (CallFunction|TurnHand true)
    (Utilities|Time|SetTimerbyEvent (delegate Custom|CheckAKey) 0.05))
  (:Released
    (Variables|Input|SetAKey false)))

(event Input|ActionEvents|InputActionRight
  (params (Key :type Key%20Structure :default "None"))
  ;[0.1692 1 0.1706] Rotate wheel to the right
  (:Pressed
    (Variables|Input|SetDKey true)
    (CallFunction|TurnHand false)
    (Utilities|Time|SetTimerbyEvent (delegate Custom|CheckDkey) 0.05))
  (:Released
    (Variables|Input|SetDKey false)))

(fn ConstructionScript
  ;[1 1 1] turn times into code
  (|CallParentFunction)
  (bind _returnvalue (CallFunction|EncodePasswords (Variables|Time|GetPasswordTime)))
  (Variables|Password|SetCorrectCode _returnvalue)
  (bind _returnvalue_2 (CallFunction|EncodePasswords (Variables|Time|GetStartTime)))
  (Variables|Password|SetStartCode _returnvalue_2))

(fn TurnHand
  (params (Clockwise? :type Boolean))
  ;[1 1 1] change input code and send data to animation blueprint
  (Variables|Password|SetCurrentCode (+ (Variables|Password|GetCurrentCode) (Math|Integer|SelectInt -1 1 Clockwise?)))
  (Default|SetHandsRotation (Variables|Refs|GetABP_ClockRef) (Variables|Password|GetCurrentCode))
  (CallFunction|ServerSetWheelRotation (Variables|Password|GetCurrentCode)))

(fn CheckPassword
  ;[1 1 1] Check if clock set to correct password
  (if (>= (Variables|Password|GetCurrentCode) 0) :!label _label
    (if (== (Math|Integer|%(Integer) (Variables|Password|GetCurrentCode) 720) (Variables|Password|GetCorrectCode))
      (CallFunction|ServerPasswordIsCorrect)
      (CallFunction|ExitPuzzle))
    (else
      (Variables|Password|SetCurrentCode (+ (Variables|Password|GetCurrentCode) 720))
      (goto _label))))

(fn ExitPuzzle
  (|CallParentFunction))

(fn ResetLock
  ;[1 1 1] Reset hands rotations
  (Default|SetHandsRotation (Variables|Refs|GetABP_ClockRef) (Variables|Password|GetStartCode))
  (Variables|Password|SetCurrentCode (Variables|Password|GetStartCode)))

(fn EncodePasswords
  (params (F_ClockTimes :type F%20Clock%20Times%20Structure%20%28by%20ref%29))
  (bind (_hour _minute) (Utilities|Struct|BreakF_ClockTimes F_ClockTimes))
  ;[1 1 1] encode times into codes
  (return (+ (* (Math|Integer|%(Integer) _hour 12) 60) _minute)))