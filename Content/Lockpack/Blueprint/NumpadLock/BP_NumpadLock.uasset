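; Numpad lock puzzle, built on a parent puzzle class, that opens a target door when the correct code is entered.
; WASD moves a cube highlight between key sockets via neighbor maps; Space presses the key through the AnimBP, with shortcuts for check, delete, reset and exit.
; Digits fill an array shown on a TextRender display and compared locally to the password.
; Server events multicast success or a brief input-blocking error, with sound and material feedback.
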(event Custom|Server_PasswordIsCorrect
  ;[0 0.7563 1] Password is correct
  (CallFunction|MultiCastCorrectPassword)
  (Collision|SetCollisionEnabled (Variables|Default|GetSphere) "NoCollision"))

(event Custom|Server_PasswordISWrong
  (CallFunction|MulticastErrorPopUp))

(event Custom|MultiCast_CorrectPassword
  (bind _textrender (Variables|Default|GetTextRender))
  ;[0 0.7563 1] Multicast Open safe lock door
  (Rendering|Material|SetScalarParameterValueonMaterials (Variables|Default|GetSkeletalMesh) "NumSwitch" 1.0)
  (Rendering|Components|TextRender|SetWorldSize _textrender 2e+01)
  (Rendering|Components|TextRender|SetText _textrender (Utilities|Text|MakeLiteralText "HELLO"))
  (Rendering|Components|TextRender|SetTextRenderColor _textrender (Variables|Colors|GetCorrectColor))
  (Audio|PlaySound2D (Variables|Sound|GetCorrectSound) 1.0 1.0 0.0 0 0)
  (CallFunction|MulticastOpenTargetDoor 0.0))

(event Custom|ErrorPopUp
  (CallFunction|ShowError)
  (Utilities|FlowControl|Delay 0.2)
  (CallFunction|HideError))

(event Custom|Multicast_ErrorPopUp
  (CallFunction|ErrorPopUp))

(event EventBeginPlay
  ;[1 1 1] Override begin play
  (|CallParentFunction)
  (bind _asabp_numpad_lock (Utilities|Casting|CastToABP_NumpadLock (Components|SkeletalMesh|GetAnimInstance (Variables|Default|GetSkeletalMesh)))
    (:then
      (Variables|References|SetABP_NumpadLockRef _asabp_numpad_lock))
    (:CastFailed
      _))
  (Variables|Password|SetPasswordLength (Utilities|Array|Length (Variables|Password|GetPassword)))
  (CallFunction|ClearPassword))

(event EventClientEnterPuzzle
  (params (Character :type Character%20Object%20Reference))
  ;[0.01096 0.1119 0.1356] On entering puzzle, After call parent version, set show wheel to first one
  (|CallParentFunction Character)
  (Rendering|SetVisibility (Variables|Default|GetCube) true false)
  (CallFunction|SetKeyLocation (Variables|Keypad|GetSelectedKey)))

(event Input|KeyboardEvents|A
  (params (Key :type Key%20Structure :default "None"))
  ;[0.1692 1 0.1706] Select New Key
  (:Pressed
    (CallFunction|ChangeSelection "NewEnumerator3")))

(event Input|KeyboardEvents|D
  (params (Key :type Key%20Structure :default "None"))
  ;[0.1692 1 0.1706] Select New Key
  (:Pressed
    (CallFunction|ChangeSelection "NewEnumerator1")))

(event Input|KeyboardEvents|Enter
  (params (Key :type Key%20Structure :default "None"))
  ;[0.1692 1 0.1706] Check Password puzzle
  (:Pressed
    (CallFunction|CheckPassword)))

(event Input|KeyboardEvents|S
  (params (Key :type Key%20Structure :default "None"))
  ;[0.1692 1 0.1706] Select New Key
  (:Pressed
    (CallFunction|ChangeSelection "NewEnumerator2")))

(event Input|KeyboardEvents|W
  (params (Key :type Key%20Structure :default "None"))
  ;[0.1692 1 0.1706] Select New Key
  (:Pressed
    (CallFunction|ChangeSelection "NewEnumerator0")))

(event Input|KeyboardEvents|F
  (params (Key :type Key%20Structure :default "None"))
  ;[0.1692 1 0.1706] Exit puzzle
  (:Pressed
    (CallFunction|ExitPuzzle)))

(event Input|KeyboardEvents|R
  (params (Key :type Key%20Structure :default "None"))
  ;[0.1692 1 0.1706] ResetLock
  (:Pressed
    (if (Variables|Keypad|GetbCanPressKey)
      (CallFunction|ClearPassword))))

(event Input|KeyboardEvents|SpaceBar
  (params (Key :type Key%20Structure :default "None"))
  ;[0.1692 1 0.1706] Check if password is correct
  (:Pressed
    (if (Variables|Keypad|GetbCanPressKey)
      (CallFunction|EnterDigit))))

(event Input|KeyboardEvents|Backspace
  (params (Key :type Key%20Structure :default "None"))
  ;[0.1692 1 0.1706] Delete Character on puzzle
  (:Pressed
    (CallFunction|DeleteCharacter)))

(fn ConstructionScript
  (|CallParentFunction))

(fn SetKeyLocation
  (params (Key :type Integer%20%28by%20ref%29))
  ;[1 1 1] Set the location of the indicator
  (Transformation|SetWorldLocation (Variables|Default|GetCube) (.location (Transformation|GetSocketTransform (Variables|Default|GetSkeletalMesh) (.Value (Utilities|Map|Find (Variables|Keypad|GetNumberKeyToBoneName) Key)) "RTS_World")) false true))

(fn UpdateLCD
  ;[1 1 1] Write the packs of digits each time a key is entered
  (for _array_element (Variables|Password|GetEnteredKey)
    (if (!= _array_element -1)
      (LocalVariables|SetLCD (Utilities|String|Append (LocalVariables|GetLCD) (Utilities|String|ToString(Integer) _array_element)))))
  (Rendering|Components|TextRender|SetText (Variables|Default|GetTextRender) (Utilities|Text|ToText(String) (LocalVariables|GetLCD))))

(fn ClearPassword
  (for (_ _array_index) (Variables|Password|GetPassword)
    (Utilities|Array|SetArrayElem (Variables|Password|GetEnteredKey) _array_index -1 true)
    (Variables|Password|SetIndex 0)
    (CallFunction|UpdateLCD)))

(fn DeleteCharacter
  ;[1 1 1] Its works like backspace
  (Variables|Password|SetIndex (Math|Integer|SelectInt 0 (- (Variables|Password|GetIndex) 1) (<= (Variables|Password|GetIndex) 0)))
  (Utilities|Array|SetArrayElem (Variables|Password|GetEnteredKey) (Variables|Password|GetIndex) -1)
  (CallFunction|UpdateLCD))

(fn ChangeSelection
  (params (Direction :type E_Direction%20Enum :default "NewEnumerator0"))
  ;[1 1 1] Find next highlighted key by pressing arrow keys
  (bind _output_get (Variables|Keypad|SetSelectedKey (.Value (Utilities|Map|Find (Utilities|Select :Index Direction :NewEnumerator0 (Variables|Keypad|GetTop) :NewEnumerator1 (Variables|Keypad|GetRight) :NewEnumerator2 (Variables|Keypad|GetBot) :NewEnumerator3 (Variables|Keypad|GetLeft)) (Variables|Keypad|GetSelectedKey)))))
  (CallFunction|SetKeyLocation _output_get))

(fn ExitPuzzle
  ;[1 1 1] Override Exit puzzle
  (|CallParentFunction)
  (Rendering|SetVisibility (Variables|Default|GetCube) false false)
  (Variables|Keypad|SetSelectedKey 1))

(fn CheckPassword
  ;[1 1 1] Check each digit with correct password
  (bind (_array_element _array_index) (Utilities|Array|ForEachLoopwithBreak (Variables|Password|GetPassword) :!label _label)
    (:LoopBody
      (if (not (== _array_element (Utilities|Array|Get(acopy) (Variables|Password|GetEnteredKey) _array_index)))
        (LocalVariables|SetbPasswordIsCorrect false)
        (goto _label Break)))
    (:Completed
      (if (LocalVariables|GetbPasswordIsCorrect)
        (CallFunction|ServerPasswordIsCorrect)
        (Utilities|Time|SetTimerbyFunctionName 0 "ExitPuzzle" 1.5)
        (else
          (CallFunction|ServerPasswordISWrong))))))

(fn EnterDigit
  ;[1 1 1] Find whick key is pressed
  (Audio|PlaySound2D (Variables|Sound|GetEnterSound) 1.0 1.0 0.0 0 0)
  (Default|KeyPressed (Variables|References|GetABP_NumpadLockRef) (Variables|Keypad|GetSelectedKey))
  (switch int (Variables|Keypad|GetSelectedKey)
    (:0
      (if (< (Variables|Password|GetIndex) (Variables|Password|GetPasswordLength)) :!label _label
        ;[1 1 1] Add New Number
        (Utilities|Array|SetArrayElem (Variables|Password|GetEnteredKey) (Variables|Password|GetIndex) (Variables|Keypad|GetSelectedKey) true)
        (Math|Integer|IncrementInt (Variables|Password|GetIndex)
          (:%20%20
            (CallFunction|UpdateLCD)))))
    (:1
      (goto _label))
    (:2
      (goto _label))
    (:3
      (goto _label))
    (:4
      (goto _label))
    (:5
      (goto _label))
    (:6
      (goto _label))
    (:7
      (goto _label))
    (:8
      (goto _label))
    (:9
      (goto _label))
    (:10
      (CallFunction|ClearPassword))
    (:12
      (CallFunction|DeleteCharacter))
    (:13
      (CallFunction|CheckPassword))))

(fn ShowError
  ;[1 1 1] Show Error
  (Rendering|Components|TextRender|SetTextRenderColor (Variables|Default|GetTextRender) (Variables|Colors|GetErrorColor))
  (Rendering|Components|TextRender|SetText (Variables|Default|GetTextRender) (Utilities|Text|MakeLiteralText "Error"))
  (Rendering|Material|SetScalarParameterValueonMaterials (Variables|Default|GetSkeletalMesh) "NumSwitch" -1.0)
  (Variables|Keypad|SetbCanPressKey false)
  (Audio|PlaySound2D (Variables|Sound|GetErrorSound) 1.0 1.0 0.0 0 0))

(fn HideError
  ;[1 1 1] Hide Error
  (Rendering|Components|TextRender|SetTextRenderColor (Variables|Default|GetTextRender) (Variables|Colors|GetDefaultColor))
  (CallFunction|ClearPassword)
  (Variables|Keypad|SetbCanPressKey true)
  (Rendering|Material|SetScalarParameterValueonMaterials (Variables|Default|GetSkeletalMesh) "NumSwitch" 0.0))