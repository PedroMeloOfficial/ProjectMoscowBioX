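; Base actor for networked lock puzzles, which players enter through interaction and which open a target actor when solved.
; Interacting with an unowned lock makes the character its owner, then a client RPC blends to the lock's camera, moves input to it and shows a guide widget.
; Exiting restores the player and clears ownership on the server.
; A solve multicast marks it solved and calls the target's "Open" by timer.
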(event OnComponentBeginOverlap(Sphere)
  (params (OverlappedComponent :type Primitive%20Component%20Object%20Reference) (OtherActor :type Actor%20Object%20Reference) (OtherComp :type Primitive%20Component%20Object%20Reference) (OtherBodyIndex :type Integer) (bFromSweep :type Boolean) (SweepResult :type Hit%20Result%20Structure%20%28by%20ref%29))
  ;[1 1 1] OverlapWithCharacter
)

(event OnComponentEndOverlap(Sphere)
  (params (OverlappedComponent :type Primitive%20Component%20Object%20Reference) (OtherActor :type Actor%20Object%20Reference) (OtherComp :type Primitive%20Component%20Object%20Reference) (OtherBodyIndex :type Integer))
  ;[1 1 1] OverlapWithCharacter
)

(event Custom|Multicast_OpenTargetDoor
  (params (StartDelay :type Float%20%28double-precision%29))
  ;[1 1 1] On passwordCorrect entered
  (Variables|Default|SetIsSolved true)
  (bind _opentarget (Variables|Default|GetOpenTarget)
    (:then
      (Utilities|Time|SetTimerbyFunctionName _opentarget "Open" (Math|Float|Max(Float) StartDelay 0.1)))
    (:else)))

(event Custom|Server_ExitPuzzle
  ;[0 0.7563 1] Set the required settings for the puzzle
  (Actor|SetOwner 0)
  (Variables|Default|SetIsOnPuzzle false))

(event Custom|Multicast_PauseAnim
  (params (Pause%20Anims :type Boolean))
  ;[0 0.7563 1] Pause Animation for performance
  (Variables|/Script/Engine.SkeletalMeshComponent|SetbPauseAnims (Variables|Default|GetSkeletalMesh) Pause%20Anims))

(event Custom|Client_EnterPuzzle
  (params (Character :type Character%20Object%20Reference))
  ;[0 0.7563 1] enter to the camera
  ; enable input to turn it
  (bind _output_get (Variables|Default|SetCharacterRef Character))
  (Development|SetHiddeninGame (Variables|/Script/Engine.Character|GetMesh _output_get) true true)
  (bind _asplayer_controller (Utilities|Casting|CastToPlayerController (Pawn|GetController _output_get)))
  (Variables|Default|SetPlayerControllerRef _asplayer_controller)
  (CallFunction|EnterCamera)
  (Input|EnableInput (Variables|Default|GetPlayerControllerRef))
  (Input|DisableInput (Variables|Default|GetCharacterRef) (Variables|Default|GetPlayerControllerRef))
  (Development|SetHiddeninGame (Variables|Default|GetWidget) true false)
  (Variables|Default|SetIsOnPuzzle true))

(event EventBeginPlay
  ;[1 1 1] Begin Play
  (Networking|SwitchHasAuthority
    (:Authority
      (Collision|SetCollisionEnabled (Variables|Default|GetSphere) "QueryOnly"))))

(event EventInteractWIthCharacter
  (params (Character :type Character%20Object%20Reference))
  ;[0.956 1 0.4233] Comment
  (if (not (Utilities|IsValid (Components|GetOwner)))
    (CallFunction|EnterPuzzle Character)))

(event EventInterfaceToggleFocus
  (params (Focus :type Boolean))
  (bind _widget (Variables|Default|GetWidget))
  ;[0 0 0 0.5] Interaction integration to display the interaction widget
  (if (not (Variables|Default|GetIsSolved))
    (if (not (Variables|Default|GetIsOnPuzzle))
      (Development|SetHiddeninGame _widget (not Focus) false)
      (if (Rendering|IsVisible _widget)
        (bind _asui_interaction (Utilities|Casting|CastToUI_Interaction (UserInterface|GetWidget _widget)))
        (bind _output_get (Variables|Default|SetAs%20UI%20Interaction _asui_interaction))
        (Rendering|Components|TextRender|SetText (Variables|/Game/BodycamFPSKIT/Blueprints/Widgets/UI_Interaction.UI_Interaction_C|GetItemName _output_get) (Variables|Default|GetName)) ; ITEM NAME
      ))))

(fn ConstructionScript)

(fn EnterPuzzle
  (params (Character :type Character%20Object%20Reference))
  (Actor|SetOwner Character)
  (CallFunction|MulticastPauseAnim false)
  (CallFunction|ClientEnterpuzzle Character))

(fn EnterCamera
  ;[1 1 1] Enter the Safe Camera
  (bind _playercontrollerref (Variables|Default|GetPlayerControllerRef)
    (:then
      (Game|Player|SetViewTargetwithBlend _playercontrollerref self 0.0 "VTBlend_Linear" 0.0 false)
      (Utilities|FlowControl|Sequence
        (:then_0
          (bind _interactwidget (Variables|Default|GetInteractWIdget)
            (:then
              (Widget|RemovefromParent _interactwidget)
              (Variables|Default|SetInteractWIdget 0))
            (:else)))
        (:then_1
          (bind _guidwidget (Variables|Default|GetGuidWidget)
            (:then
              (Widget|RemovefromParent _guidwidget))
            (:else
              _))
          (bind _returnvalue (UserInterface|CreateWidget (Variables|Default|GetGuidWidgetClass)))
          (Variables|Default|SetGuidWidget _returnvalue)
          (bind _guidwidget_2 (Variables|Default|GetGuidWidget)
            (:then
              (UserInterface|Viewport|AddtoViewport _guidwidget_2 0))
            (:else)))))
    (:else)))

(fn ExitCamera
  (bind _playercontrollerref (Variables|Default|GetPlayerControllerRef))
  (bind _characterref (Variables|Default|GetCharacterRef))
  ;[1 1 1] Exit the Camera and return to the main player
  (if (and (Utilities|IsValid _playercontrollerref) (Utilities|IsValid _characterref))
    (Game|Player|SetViewTargetwithBlend _playercontrollerref _characterref 0.0 "VTBlend_Linear" 0.0 false)))

(fn ExitPuzzle
  ;[1 1 1] Try to exit the puzzle
  (Input|DisableInput (Variables|Default|GetPlayerControllerRef))
  (Utilities|IsValid (Variables|Default|GetCharacterRef)
    (:Is%20Valid
      (Input|EnableInput (Variables|Default|GetCharacterRef) (Variables|Default|GetPlayerControllerRef))
      (Development|SetHiddeninGame (Variables|/Script/Engine.Character|GetMesh (Variables|Default|GetCharacterRef)) false true)
      (CallFunction|ExitCamera)
      (Variables|Default|SetCharacterRef 0)
      (Variables|Default|SetPlayerControllerRef 0)
      (CallFunction|ServerExitPuzzle)
      (bind _guidwidget (Variables|Default|GetGuidWidget)
        (:then
          (Widget|RemovefromParent _guidwidget)
          (Variables|Default|SetGuidWidget 0))
        (:else)))))

(fn InteractionWidgetRef
  (return 0))