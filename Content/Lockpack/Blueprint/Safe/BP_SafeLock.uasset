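; BP_SafeLock is a multiplayer combination-safe puzzle that one player at a time operates through its own camera and widget.
; Interacting makes that character the owner, then a client event moves input and view to the safe.
; The client turns the dial and tracks three numbers in alternating directions, resetting progress on a wrong direction.
; Server-to-multicast events replicate wheel rotation, resets and door opening through the safe's AnimBP, with correctness decided client-side.
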(event Custom|Server_PasswordIsCorrect
  ;[0 0.7563 1] Password is correct
  (CallFunction|MultiCastOpenDoor)
  (Collision|SetCollisionEnabled (Variables|Default|GetSphere) "NoCollision"))

(event Custom|server_SetWheelRotation
  (params (Rotation :type Float%20%28single-precision%29))
  ;[0 0.7563 1] Set Rotation for server
  (CallFunction|MulticastSetWheelRotation Rotation))

(event Custom|MultiCast_OpenDoor
  ;[0 0.7563 1] Multicast Open safe lock door
  (Default|OpenDoor (Variables|References|GetABPSafeRef)))

(event Custom|Server_ExitPuzzle
  ;[0 0.7563 1] Set the required settings for the puzzle
  (Actor|SetOwner 0))

(event Custom|Multicast_SetWheelRotation
  (params (Rotation :type Float%20%28single-precision%29))
  ;[0 0.7563 1] Set Rotation for server
  (Default|SetWheelRotation (Variables|References|GetABPSafeRef) Rotation))

(event Custom|Multicast_PauseAnim
  (params (Pause%20Anims :type Boolean))
  ;[0 0.7563 1] Comment
  (Variables|/Script/Engine.SkeletalMeshComponent|SetbPauseAnims (Variables|Default|GetSkeletalMesh) Pause%20Anims))

(event Custom|Multicast_ResetLock
  ;[0 0.7563 1] Reset lock position for all players
  ; it also returns to the interacted player but will override the current
  (Password|ResetLock))

(event Custom|Server_ResetLock
  ;[0 0.7563 1] Reset lock position for all players
  ; it also returns to the interacted player but will override the current
  (CallFunction|MulticastResetLock))

(event Custom|Client_EnterPuzzle
  (params (Character :type Character%20Object%20Reference))
  ;[0 0.7563 1] enter to the camera
  ; enable input to turn it
  (bind _output_get (Variables|References|SetCharacterRef Character))
  (bind _asplayer_controller (Utilities|Casting|CastToPlayerController (Pawn|GetController _output_get)))
  (Variables|References|SetPlayerControllerRef _asplayer_controller)
  (Camera|EnterCamera)
  (Input|EnableInput (Variables|References|GetPlayerControllerRef))
  (Input|DisableInput (Variables|References|GetCharacterRef) (Variables|References|GetPlayerControllerRef))
  (UserInterface|Viewport|AddtoViewport (Variables|References|GetWidgetRef) 0))

(event Custom|CheckDKey
  ;[0.1692 1 0.1706] Turn By Key
  (if (Variables|Input|GetDKey)
    (Password|TurnWheel false)))

(event Custom|CheckAKey
  ;[0.1692 1 0.1706] Turn By Key
  (if (Variables|Input|GetAKey)
    _))

(event EventBeginPlay
  ;[1 1 1] Begin Play
  (bind _asabp_safe (Utilities|Casting|CastToABP_Safe (Components|SkeletalMesh|GetAnimInstance (Variables|Default|GetSkeletalMesh)))
    (:then
      (Variables|References|SetABPSafeRef _asabp_safe))
    (:CastFailed
      _))
  (bind _aswbp_safe_lock_widget (Utilities|Casting|CastToWBP_SafeLockWidget (UserInterface|GetUserWidgetObject (Variables|Default|GetWidget)))
    (:then
      (Variables|References|SetWidgetRef _aswbp_safe_lock_widget))
    (:CastFailed
      _))
  (Networking|SwitchHasAuthority
    (:Authority
      (Collision|SetCollisionEnabled (Variables|Default|GetSphere) "QueryOnly"))))

(event EventInteractWIthCharacter
  (params (Character :type Character%20Object%20Reference))
  ;[0.958 1 0.4223] EnterPuzzle
  (if (not (Utilities|IsValid (Components|GetOwner)))
    (Puzzle|EnterPuzzle Character)))

(event Input|ActionEvents|InputActionLeft
  (params (Key :type Key%20Structure :default "None"))
  ;[0.1692 1 0.1706] Turn By Key
  (:Pressed
    (Variables|Input|SetAKey true)
    (Password|TurnWheel true)
    (Utilities|Time|SetTimerbyEvent (delegate Custom|CheckAKey) 0.2))
  (:Released
    (Variables|Input|SetAKey false)))

(event Input|ActionEvents|InputActionRight
  (params (Key :type Key%20Structure :default "None"))
  ;[0.1692 1 0.1706] Turn By Key
  (:Pressed
    (Variables|Input|SetDKey true)
    (Password|TurnWheel false))
  (:Released
    (Variables|Input|SetDKey false)))

(event Input|ActionEvents|InputActionInteract
  (params (Key :type Key%20Structure :default "None"))
  ;[0.1692 1 0.1706] Disable the input in the client and set settings to ExitPuzzle on server
  (:Pressed
    (Puzzle|ExitPuzzle)))

(event Input|ActionEvents|InputActionAcceptKey
  (params (Key :type Key%20Structure :default "None"))
  ;[0.1692 1 0.1706] Check Password key
  (:Pressed
    (Password|CheckPasswordCombie)))

(event Input|ActionEvents|InputActionReset
  (params (Key :type Key%20Structure :default "None"))
  ;[0.1692 1 0.1706] Reset
  (:Pressed
    (Input|DisableInput (Variables|References|GetPlayerControllerRef))
    (Utilities|Time|SetTimerbyFunctionName 0 "Reenable Input" 1.5)
    (Password|ResetLock)
    (Audio|PlaySound2D (Variables|Sound|GetResetSound) 1.0 1.0 0.0 0 0)
    (CallFunction|ServerResetLock)))

(event Input|MouseEvents|MouseWheelUp
  (params (Key :type Key%20Structure :default "None"))
  ;[0.1692 1 0.1706] Turn By Wheel
  (:Pressed
    (Password|TurnWheel false)))

(event Input|MouseEvents|MouseWheelDown
  (params (Key :type Key%20Structure :default "None"))
  ;[0.1692 1 0.1706] Turn By Wheel
  (:Pressed
    (Password|TurnWheel false)))

(fn ConstructionScript)

(fn ReenableInput
  ;[1 1 1] This function is called by timer
  ; reenable the input
  (Input|EnableInput (Variables|References|GetPlayerControllerRef)))

(fn CheckPasswordProcess
  ;[1 1 1] Check if reached correct number in the correct direction
  (if (>= (Variables|Password|GetsuccessStage) 3)
    (Variables|Password|SetsuccessStage 0 :!label _label)
    (elif (Math|Boolean|Equal(Boolean) (Variables|WheelRotation|GetbIsClockWise) (Utilities|Select :Index (Variables|Password|GetsuccessStage) :Option%200 false :Option%201 true :Option%202 false))
      (if (== (Utilities|Select :Index (Variables|Password|GetsuccessStage) :Option%200 (Variables|Password|GetPassPhase1) :Option%201 (Variables|Password|GetPassPhase2) :Option%202 (Variables|Password|GetPassPhase3)) (Variables|WheelRotation|GetInsertedNumber))
        ;[1 1 1] Increase success stage
        (Math|Integer|IncrementInt (Variables|Password|GetsuccessStage)
          (:%20%20
            (Audio|PlaySound2D (Variables|Sound|GetCorrectkeySound) 0.3 1.0 0.0 0 0))))
      (else
        (goto _label)))))

(fn TurnWheel
  (params (Clockwise? :type Boolean))
  ;[1 1 1] Change the wheel by 6degree then password proccess
  (Variables|Password|SetRotationChanged (Class|KismetMathLibrary|XORBoolean Clockwise? (Variables|WheelRotation|GetbIsClockWise)))
  (Variables|WheelRotation|SetbIsClockWise Clockwise?)
  (bind _output_get (Variables|WheelRotation|SetRotation (+ (Variables|WheelRotation|GetRotation) (Math|Float|SelectFloat -6.0 6.0 Clockwise?))))
  (Default|SetWheelRotation (Variables|References|GetABPSafeRef) _output_get)
  (CallFunction|ServerSetWheelRotation (Variables|WheelRotation|GetRotation))
  (bind _output_get_2 (Variables|WheelRotation|SetInsertedNumber (Math|Float|Truncate (/ (Class|KismetMathLibrary|ClampAxis (Variables|WheelRotation|GetRotation)) 6.0))))
  (Default|UpdateWidgetNumber (Variables|References|GetWidgetRef) _output_get_2 (Variables|Password|GetRotationChanged))
  (Password|CheckPasswordProcess)
  (Audio|PlaySound2D (Variables|Sound|GetSwitch02) 1.0 1.0 0.0 0 0))

(fn ResetLock
  ;[1 1 1] Set this for  current player for real time respond
  (Default|ResetWheelRotation (Variables|References|GetABPSafeRef) (Variables|WheelRotation|GetRotation))
  (Variables|WheelRotation|SetRotation 0.0)
  (Variables|WheelRotation|SetbIsClockWise false)
  (Default|Reset (Variables|References|GetWidgetRef)))

(fn CheckPasswordCombie
  ;[1 1 1] Check if password is correct then send the sresult to the server if it was correct
  (if (== (Variables|Password|GetsuccessStage) 3)
    (CallFunction|ServerPasswordIsCorrect)
    (Puzzle|ExitPuzzle)))

(fn ExitCamera
  (bind _playercontrollerref (Variables|References|GetPlayerControllerRef))
  (bind _characterref (Variables|References|GetCharacterRef))
  ;[1 1 1] Exit the Camera and return to the main player
  (if (and (Utilities|IsValid _playercontrollerref) (Utilities|IsValid _characterref))
    (Game|Player|SetViewTargetwithBlend _playercontrollerref _characterref 0.1 "VTBlend_Linear" 0.0 false)))

(fn EnterCamera
  ;[1 1 1] Enter the Safe Camera
  (bind _playercontrollerref (Variables|References|GetPlayerControllerRef)
    (:then
      (Game|Player|SetViewTargetwithBlend _playercontrollerref self 0.1 "VTBlend_Linear" 0.0 false))
    (:else)))

(fn ExitPuzzle
  ;[1 1 1] Try to exit the puzzle
  (Input|DisableInput (Variables|References|GetPlayerControllerRef))
  (Input|EnableInput (Variables|References|GetCharacterRef) (Variables|References|GetPlayerControllerRef))
  (Password|ResetLock)
  (Camera|ExitCamera)
  (Variables|References|SetCharacterRef 0)
  (Variables|References|SetPlayerControllerRef 0)
  (Widget|RemovefromParent (Variables|References|GetWidgetRef))
  (CallFunction|ServerExitPuzzle))

(fn EnterPuzzle
  (params (Character :type Character%20Object%20Reference))
  (Actor|SetOwner Character)
  (CallFunction|MulticastPauseAnim false)
  (CallFunction|ClientEnterpuzzle Character))