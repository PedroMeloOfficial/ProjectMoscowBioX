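; Directional combination lock puzzle where players enter a sequence of up, right, down and left handle moves to open a target door.
; Construction converts Password into integer codes, compared against rate-limited inputs once the entered length matches.
; A wrong code either auto-resets or flags a required reset in the guide widget.
; Handle animation plays locally and, like opening and reset montages, replicates through server-to-multicast events.
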(event Custom|Server_PasswordIsCorrect
  ;[0 0.7563 1] Password is correct
  (CallFunction|MultiCastOpenDoor)
  (Collision|SetCollisionEnabled (Variables|Default|GetSphere) "NoCollision"))

(event Custom|Server_AnimationMoveHand
  (params (Direction :type E_Direction%20Enum :default "NewEnumerator0"))
  ;[0 0.7563 1] Set wheel Rotation for all players
  (CallFunction|MulticastAnimationMoveHand Direction))

(event Custom|MultiCast_OpenDoor
  ;[0 0.7563 1] Multicast Open safe lock door
  (Utilities|FlowControl|Delay 0.2)
  (Animation|Montage|PlayMontage (Variables|Default|GetSkeletalMesh) (Variables|Montages|GetOpenMontage)
    (:then
      (Audio|PlaySoundatLocation (Variables|Sound|GetOpenSound) (Transformation|GetActorLocation) "0, 0, 0" 1.0 1.0 0.0 0 0 0)
      (CallFunction|MulticastOpenTargetDoor 0.0))))

(event Custom|Multicast_AnimationMoveHand
  (params (Direction :type E_Direction%20Enum :default "NewEnumerator0"))
  ;[0 0.7563 1] Set wheel Rotation for all players
  (Default|AnimationMoveHand (Variables|Refs|GetABP_ClockRef) Direction))

(event Custom|Server_PlayResetLock
  ;[0 0.7563 1] Restart lock for all players
  (CallFunction|MulticastPlayResetLock))

(event Custom|Multicast_PlayResetLock
  ;[0 0.7563 1] Restart lock for all players
  (Animation|Montage|PlayMontage (Variables|Default|GetSkeletalMesh) (Variables|Montages|GetResetMontage)))

(event EventBeginPlay
  ;[1 1 1] Override begin play
  (|CallParentFunction)
  (bind _asabp_directional_lock (Utilities|Casting|CastToABP_DirectionalLock (Components|SkeletalMesh|GetAnimInstance (Variables|Default|GetSkeletalMesh))))
  (Variables|Refs|SetABP_ClockRef _asabp_directional_lock))

(event Input|ActionEvents|InputActionReset
  (params (Key :type Key%20Structure :default "None"))
  ;[0.1692 1 0.1706] ResetLock
  (:Pressed
    (CallFunction|ResetLock)))

(event Input|ActionEvents|InputActionUp
  (params (Key :type Key%20Structure :default "None"))
  ;[0.1692 1 0.1706] Rotate wheel to the left
  (:Pressed
    (if (Variables|Input|GetbCanPressKey)
      (Variables|Input|SetbCanPressKey false)
      (CallFunction|MoveHandle "NewEnumerator0"))))

(event Input|ActionEvents|InputActionRight
  (params (Key :type Key%20Structure :default "None"))
  ;[0.1692 1 0.1706] Rotate wheel to the left
  (:Pressed
    (if (Variables|Input|GetbCanPressKey)
      (Variables|Input|SetbCanPressKey false)
      (CallFunction|MoveHandle "NewEnumerator1"))))

(event Input|ActionEvents|InputActionDown
  (params (Key :type Key%20Structure :default "None"))
  ;[0.1692 1 0.1706] Rotate wheel to the left
  (:Pressed
    (if (Variables|Input|GetbCanPressKey)
      (Variables|Input|SetbCanPressKey false)
      (CallFunction|MoveHandle "NewEnumerator2"))))

(event Input|ActionEvents|InputActionLeft
  (params (Key :type Key%20Structure :default "None"))
  ;[0.1692 1 0.1706] Rotate wheel to the left
  (:Pressed
    (if (Variables|Input|GetbCanPressKey)
      (Variables|Input|SetbCanPressKey false)
      (CallFunction|MoveHandle "NewEnumerator3"))))

(event Input|ActionEvents|InputActionAcceptKey
  (params (Key :type Key%20Structure :default "None"))
  ;[0.1692 1 0.1706] Check if password is correct
  (:Pressed
    (CallFunction|CheckPassword)))

(event Input|ActionEvents|InputActionInteract
  (params (Key :type Key%20Structure :default "None"))
  ;[0.1692 1 0.1706] Exit puzzle
  (:Pressed
    (CallFunction|ExitPuzzle)))

(fn ConstructionScript
  ;[1 1 1] turn times into code
  (|CallParentFunction)
  (for (_array_element _array_index) (Variables|Password|GetPassword)
    (Utilities|Array|SetArrayElem (Variables|Password|GetCorrectPassword) _array_index (Math|Conversions|ToInteger(Byte) _array_element) true)))

(fn CheckPassword
  ;[1 1 1] Check if clock set to correct password
  (if (== (Utilities|Array|Length (Variables|Password|GetCorrectPassword)) (Utilities|Array|Length (Variables|Password|GetEnteredPassword)))
    (for (_array_element _array_index) (Variables|Password|GetCorrectPassword)
      (LocalVariables|SetbPasswordIsCorrect (and (== _array_element (Utilities|Array|Get(acopy) (Variables|Password|GetEnteredPassword) _array_index)) (LocalVariables|GetbPasswordIsCorrect))))
    ;[1 1 1] Continue with correct password
    (if (and (not (Variables|Password|GetbResetNeeded)) (LocalVariables|GetbPasswordIsCorrect))
      (CallFunction|ServerPasswordIsCorrect)
      (CallFunction|ExitPuzzle)
      (else
        ;[1 1 1] Check if auto restart is activated
        (Audio|PlaySound2D (Variables|Sound|GetIncorrectSound) 1.0 1.0 0.0 0 0)
        (if (Variables|Password|GetbAutoResetLock)
          (CallFunction|ResetLock)
          (else
            (CallFunction|SetResetNeeded true)))))))

(fn ExitPuzzle
  (|CallParentFunction)
  (CallFunction|ResetLock))

(fn MoveHandle
  (params (Direction :type E_Direction%20Enum :default "NewEnumerator0"))
  (bind _correctpassword (Variables|Password|GetCorrectPassword))
  (bind _returnvalue (Utilities|Array|Length _correctpassword))
  (bind _returnvalue_2 (- _returnvalue 1))
  ;[1 1 1] First Encode th input
  ; then move handle
  ; check password
  ; put key on cooldown
  (Utilities|Array|SetArrayElem (Variables|Password|GetEnteredPassword) (Variables|Password|GetIndex) (Math|Conversions|ToInteger(Byte) Direction) true)
  (bind _result (Math|Integer|IncrementInt (Variables|Password|GetIndex))
    (:%20%20
      (Variables|Password|SetIndex (select (> _result _returnvalue_2) _returnvalue_2 _result))
      (Audio|PlaySound2D (Variables|Sound|GetHandleSound) 1.0 1.0 0.0 0 0)
      (Default|AnimationMoveHand (Variables|Refs|GetABP_ClockRef) Direction)
      (CallFunction|ServerAnimationMoveHand Direction)
      (CallFunction|CheckPassword)
      (Utilities|Time|SetTimerbyFunctionName 0 "Reset Can Press Key" 0.36))))

(fn ResetLock
  ;[1 1 1] Clear the logics and play reset animation
  (Utilities|Array|Clear (Variables|Password|GetEnteredPassword))
  (Variables|Password|SetIndex 0)
  (CallFunction|SetResetNeeded false)
  (CallFunction|ServerPlayResetLock)
  (Audio|PlaySound2D (Variables|Sound|GetResetSound) 1.0 1.0 0.0 0 0))

(fn ResetCanPressKey
  (Variables|Input|SetbCanPressKey true))

(fn SetResetNeeded
  (params (ResetNeeded :type Boolean))
  ;[1 1 1] Active Reset needed to true and show the widget
  (Variables|Password|SetbResetNeeded ResetNeeded)
  (bind _aswbp_direction_lock (Utilities|Casting|CastToWBP_DirectionLock (Variables|Default|GetGuidWidget)))
  (Default|ShowResetNeeded _aswbp_direction_lock ResetNeeded))