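; BP_PuzzleDirectionDoor is a Lockpack open target: a door made of cube meshes that collapses when its puzzle password is entered correctly.
; Its Open event calls EnablePhysics, which turns on physics simulation for all the cubes.
; After a short delay the whole actor destroys itself, clearing the debris.
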(event Custom|EnablePhysics
  ;[1 1 1] Enable dop boxs when password entered correctly
  (Physics|SetSimulatePhysics (Variables|Default|GetSM_Cube15) true)
  (Utilities|FlowControl|Delay 7.0)
  (Actor|DestroyActor))

(event Custom|Open
  (CallFunction|EnablePhysics))

(fn ConstructionScript)